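; BP_door_schmal is a door actor that opens and closes automatically as BP_Player enters and leaves its overlap area.
; Overlap events play the open or close animation on the Door02 mesh, unless the DestroyedDoor flag is set.
; The Collider turns off collision half a second after opening starts and switches to QueryAndProbe as soon as closing starts.
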(event Collision|EventActorBeginOverlap
  (params (OtherActor :type Actor%20Object%20Reference))
  (Utilities|Casting|CastToBP_Player OtherActor)
  (if (not (Variables|Default|GetDestroyedDoor))
    (Components|Animation|PlayAnimation (Variables|Default|GetDoor_02) "/Game/Asseds/Blockaut/01/door/Door_02_Anim_Door_Armature_DoorAction_Open.Door_02_Anim_Door_Armature_DoorAction_Open" false)
    (Utilities|FlowControl|Delay 0.5)
    (Collision|SetCollisionEnabled (Variables|Default|GetCollider) "NoCollision")))

(event Collision|EventActorEndOverlap
  (params (OtherActor :type Actor%20Object%20Reference))
  (Utilities|Casting|CastToBP_Player OtherActor)
  (if (not (Variables|Default|GetDestroyedDoor))
    (Components|Animation|PlayAnimation (Variables|Default|GetDoor_02) "/Game/Asseds/Blockaut/01/door/Door_02_Anim_Door_Armature_DoorAction_Close.Door_02_Anim_Door_Armature_DoorAction_Close" false)
    (Collision|SetCollisionEnabled (Variables|Default|GetCollider) "QueryAndProbe")))

(fn ConstructionScript)