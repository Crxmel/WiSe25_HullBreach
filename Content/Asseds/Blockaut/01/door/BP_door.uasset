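; Automatic sliding or swinging door that opens when BP_Player overlaps it and closes when they leave, unless flagged destroyed.
; Opening disables the collider after a short delay, closing restores it, and both share a debounced sound.
; A TotoDoor variant checks the player's tape, TotoRoom hole repairs and oxygen interaction state, showing MainUI text when blocked.
; Once passed, NachTotoTrigger opens it and clears TotoDoor, making it a normal door.
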(event Custom|Nach%20toto%20trigger
  (Utilities|FlowControl|Sequence
    (:then_0
      (if (not (Variables|Default|GetDestroyedDoor))
        (Components|Animation|PlayAnimation (Variables|Default|GetDoor_02) "/Game/Asseds/Blockaut/01/door/Door_02_Anim_Door_Armature_DoorAction_Open.Door_02_Anim_Door_Armature_DoorAction_Open" false)
        (Utilities|FlowControl|Sequence
          (:then_0
            (Utilities|FlowControl|Delay 0.5)
            (Collision|SetCollisionEnabled (Variables|Default|GetCollider) "NoCollision"))
          (:then_1
            (Utilities|FlowControl|DoOnce false :!label _label
              (:Completed
                (Audio|PlaySound2D "/Game/Sounds/NewFolder/sci-fi-spaceship-large-mechanical-door-close-01.sci-fi-spaceship-large-mechanical-door-close-01" 1.0 1.0 0.0 0 0)
                (Utilities|FlowControl|Delay 1.0)
                (goto _label Reset)))))))
    (:then_1
      (Utilities|FlowControl|DoOnce false
        (:Completed
          (Variables|Default|SetTotoDoor false))))))

(event Collision|EventActorBeginOverlap
  (params (OtherActor :type Actor%20Object%20Reference))
  (bind _asbp_player (Utilities|Casting|CastToBP_Player OtherActor))
  (if (Variables|Default|GetTotoDoor)
    (Utilities|IsValid (Variables|Default|GetTotoRoom)
      (:Is%20Valid
        (bind _output_get (Variables|Default|SetAs%20BP%20Player _asbp_player))
        (if (Variables|/Game/BP´s/Player/BP_Player.BP_Player_C|GetHasTape _output_get)
          (if (Variables|/Game/BP´s/Sauerstoff/BP_roomContainer.BP_RoomContainer_C|GetAreAllHolesFixed (Variables|Default|GetTotoRoom))
            (if (Variables|/Game/BP´s/Player/BP_Player.BP_Player_C|GetSauerstoffAN (Variables|Default|GetAs%20BP%20Player))
              (if (Variables|/Game/BP´s/Player/BP_Player.BP_Player_C|GetFirstInteractWithSauerstoffinteract (Variables|Default|GetAs%20BP%20Player))
                (CallFunction|NachTotoTrigger)
                (else
                  (Default|EventVisibilityTextboxFlip (Variables|/Game/BP´s/Player/BP_Player.BP_Player_C|GetMainUI (Variables|Default|GetAs%20BP%20Player)) true)
                  (Default|EventShowText (Variables|/Game/BP´s/Player/BP_Player.BP_Player_C|GetMainUI (Variables|Default|GetAs%20BP%20Player)) 20 20 0.0)))
              (else
                (CallFunction|NachTotoTrigger)))
            (else
              (Default|EventVisibilityTextboxFlip (Variables|/Game/BP´s/Player/BP_Player.BP_Player_C|GetMainUI (Variables|Default|GetAs%20BP%20Player)) true)
              (Default|EventShowText (Variables|/Game/BP´s/Player/BP_Player.BP_Player_C|GetMainUI (Variables|Default|GetAs%20BP%20Player)) 18 18 0.0)))
          (else
            (Default|EventVisibilityTextboxFlip (Variables|/Game/BP´s/Player/BP_Player.BP_Player_C|GetMainUI (Variables|Default|GetAs%20BP%20Player)) true)
            (Default|EventShowText (Variables|/Game/BP´s/Player/BP_Player.BP_Player_C|GetMainUI (Variables|Default|GetAs%20BP%20Player)) 16 16 0.0)))))
    (elif (not (Variables|Default|GetDestroyedDoor))
      (Components|Animation|PlayAnimation (Variables|Default|GetDoor_02) "/Game/Asseds/Blockaut/01/door/Door_02_Anim_Door_Armature_DoorAction_Open.Door_02_Anim_Door_Armature_DoorAction_Open" false)
      (Utilities|FlowControl|Sequence
        (:then_0
          (Utilities|FlowControl|Delay 0.5)
          (Collision|SetCollisionEnabled (Variables|Default|GetCollider) "NoCollision"))
        (:then_1
          (Utilities|FlowControl|DoOnce false :!label _label
            (:Completed
              (Audio|PlaySound2D "/Game/Sounds/NewFolder/sci-fi-spaceship-large-mechanical-door-close-01.sci-fi-spaceship-large-mechanical-door-close-01" 1.0 1.0 0.0 0 0)
              (Utilities|FlowControl|Delay 1.0)
              (goto _label Reset))))))))

(event Collision|EventActorEndOverlap
  (params (OtherActor :type Actor%20Object%20Reference))
  (Utilities|Casting|CastToBP_Player OtherActor)
  (if (not (Variables|Default|GetTotoDoor))
    (if (not (Variables|Default|GetDestroyedDoor))
      (Components|Animation|PlayAnimation (Variables|Default|GetDoor_02) "/Game/Asseds/Blockaut/01/door/Door_02_Anim_Door_Armature_DoorAction_Close.Door_02_Anim_Door_Armature_DoorAction_Close" false)
      (Collision|SetCollisionEnabled (Variables|Default|GetCollider) "QueryAndProbe")
      (Utilities|FlowControl|DoOnce false :!label _label
        (:Completed
          (Audio|PlaySound2D "/Game/Sounds/NewFolder/sci-fi-spaceship-large-mechanical-door-close-01.sci-fi-spaceship-large-mechanical-door-close-01" 1.0 1.0 0.0 0 0)
          (Utilities|FlowControl|Delay 1.0)
          (goto _label Reset))))))

(fn ConstructionScript)