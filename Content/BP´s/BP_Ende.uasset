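; BP_Ende is an end-of-game trigger actor that calls EventEndGame on a BP_Player that overlaps it.
; A BigThingRepared event latches four repair flags: Gen, Sauerstoff, Lager and Schnautze.
; The check requiring all four flags is disconnected, so the overlap ends the game regardless of repair state.
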(event Custom|BigThingRepared
  (params (Gen :type Boolean) (Sauerstoff :type Boolean) (Lager :type Boolean) (Schnautze :type Boolean))
  (Utilities|FlowControl|Sequence
    (:then_0
      (if Gen
        (Variables|Default|SetGen true)))
    (:then_1
      (if Sauerstoff
        (Variables|Default|SetSauerstoff true)))
    (:then_2
      (if Lager
        (Variables|Default|SetLager true)))
    (:then_3
      (if Schnautze
        (Variables|Default|SetSchnautze true)))))

(event Collision|EventActorBeginOverlap
  (params (OtherActor :type Actor%20Object%20Reference))
  (bind _asbp_player (Utilities|Casting|CastToBP_Player OtherActor))
  (bind _output_get (Variables|Default|SetPlayer _asbp_player))
  (Default|EventEndGame _output_get))

(fn ConstructionScript)