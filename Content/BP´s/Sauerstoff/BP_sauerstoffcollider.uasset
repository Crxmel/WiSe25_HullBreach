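; Room oxygen collider that tracks whether the player is inside and drains that room's oxygen while they are.
; Overlap hands presence over from the linked PlayerExitRoom, with a do-once that each room re-arms on its partner to block repeat triggers.
; Entry or a start-room flag starts a looping timer, skipped on entry to broken rooms.
; Each tick subtracts oxygen in proportion to holes registered through an interface, flagging empty at zero.
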(event Custom|PlayerEnterndRoom
  (Utilities|Time|SetTimerbyEvent (delegate Custom|DecreaseSauerstoff) (Variables|GameplayEinstellungen|GetTriggerTime) true))

(event Custom|DecreaseSauerstoff
  (bind _decreaseamount (Variables|GameplayEinstellungen|GetDecreaseAmount))
  (bind _holeactorlist (Variables|Default|GetHoleActorList))
  (bind _returnvalue (Utilities|Array|Length _holeactorlist))
  (bind _returnvalue_2 (* _decreaseamount _returnvalue))
  (if (not (Variables|Default|GetKeinenSauerstoffMehrImRaum))
    (if (Variables|Default|GetIsPlayerInRoom)
      (bind _output_get (Variables|GameplayEinstellungen|SetSauerstoffImRaum (- (Variables|GameplayEinstellungen|GetSauerstoffImRaum) _returnvalue_2)))
      (if (Variables|Default|GetDebug)
        (Development|PrintString (Utilities|String|Append "Sauerstoff im raum ->" (Utilities|GetDisplayName self) "    :   " (Utilities|String|ToString(Float) _output_get) "Wird abgezogen   :   " (Utilities|String|ToString(Float) _returnvalue_2)) true true "(R=0.000000,G=0.098984,B=1.000000,A=0.608696)" (- (Variables|GameplayEinstellungen|GetTriggerTime) 0.1)))
      (if (<= (Variables|GameplayEinstellungen|GetSauerstoffImRaum) 0.0)
        (Variables|GameplayEinstellungen|SetSauerstoffImRaum 0.0)
        (Variables|Default|SetKeinenSauerstoffMehrImRaum true)
        (Development|PrintString "Sauerstoff 0" true true "(R=1.000000,G=0.819493,B=0.000000,A=1.000000)")))))

(event Custom|FirstOverlapBlock
  (Utilities|FlowControl|DoOnce true) ; enters at Reset
)

(event Custom|IregestrateHole
  (params (HoleActor :type BP%20Sauerstoff%20Lag%20Parent%20Object%20Reference))
  (bind _returnvalue (Utilities|Array|Add (Variables|Default|GetHoleActorList) HoleActor))
  (if (Variables|Default|GetDebug)
    (Development|PrintString (Utilities|String|Append (Utilities|String|ToString(Integer) _returnvalue) "  ----->  " (Utilities|GetDisplayName HoleActor)) true true "(R=0.000000,G=1.000000,B=0.088261,A=1.000000)")))

(event EventBeginPlay
  (if (Variables|Default|GetRoomStart)
    (CallFunction|PlayerEnterndRoom)
    (Variables|Default|SetIsPlayerInRoom true)))

(event Collision|EventActorBeginOverlap
  (params (OtherActor :type Actor%20Object%20Reference))
  (Utilities|Casting|CastToBP_Player OtherActor)
  (Utilities|IsValid (Variables|Default|GetPlayerExitRoom)
    (:Is%20Valid
      (CallFunction|FirstOverlapBlock (Variables|Default|GetPlayerExitRoom))
      (Utilities|FlowControl|DoOnce true
        (:Completed
          (Variables|Default|SetIsPlayerInRoom true)
          (Variables|BP_sauerstoffcollider_C|SetIsPlayerInRoom (Variables|Default|GetPlayerExitRoom) false)
          (if (Variables|Default|GetDebug)
            ;[0.15 0.15 0.15 0.5] debug
            (Development|PrintString (Utilities|String|Append "Exit : " (Utilities|String|ToString(Text) (Variables|Default|GetMyRoomName)) "                 Enter : " (Utilities|String|ToString(Text) (Variables|BP_sauerstoffcollider_C|GetMyRoomName (Variables|Default|GetPlayerExitRoom)))) true true "(R=0.521266,G=1.000000,B=0.026755,A=1.000000)" 5.0))
          (if (Variables|Default|GetKaputter%20raum)
            (Development|PrintString "Raum Kaputt")
            (else
              (Utilities|FlowControl|DoOnce false
                (:Completed
                  (CallFunction|PlayerEnterndRoom))))))))))

(fn ConstructionScript)