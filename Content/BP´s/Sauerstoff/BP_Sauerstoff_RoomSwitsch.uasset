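; Overlap trigger that switches the player's current room for the oxygen (Sauerstoff) system.
; On overlap it passes the enter room to BP_Player, flips IsPlayerInRoom on the enter and exit room containers and notifies the entered room.
; A once-only gate blocks repeat triggers until re-armed via FirstOverlapBlock, which each switch calls on its linked PlaierEnterDoor.
; BeginPlay sets the player's oxygen room for the starting room one tick late.
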(event Custom|FirstOverlapBlock
  (Utilities|FlowControl|DoOnce true) ; enters at Reset
)

(event EventBeginPlay
  ;[0.15 0.15 0.15 0.5] Nur wegen first room weil BP_Player bei game start nicht gesetzt wird
  (if (Variables|/Game/BP´s/Sauerstoff/BP_RoomContainer.BP_RoomContainer_C|GetRoomStart (Variables|Default|GetPlayerEnterRoom))
    (Utilities|FlowControl|DelayUntilNextTick)
    ;;[0.15 0.15 0.15 0.5] Nimmt info ausm RoomContainer Setzt aktuellen sauerstoff im player vom Enteren Raum
    (Default|SauerstoffImRaumSet (Variables|FürFirstRoom|GetAs%20BP%20Player) (Variables|Default|GetPlayerEnterRoom))))

(event Collision|EventActorBeginOverlap
  (params (OtherActor :type Actor%20Object%20Reference))
  (Utilities|IsValid (Variables|FürFirstRoom|GetAs%20BP%20Player)
    (:Is%20Valid
      _)
    (:Is%20Not%20Valid
      (bind _asbp_player (Utilities|Casting|CastToBP_Player OtherActor))
      (Variables|FürFirstRoom|SetAs%20BP%20Player _asbp_player)))
  (Utilities|IsValid (Variables|Default|GetPlayerEnterRoom)
    (:Is%20Valid
      (CallFunction|FirstOverlapBlock (Variables|Default|GetPlaierEnterDoor))
      (Utilities|FlowControl|DoOnce true
        (:Completed
          ;[0.15 0.15 0.15 0.5] Nimmt info ausm RoomContainer Setzt aktuellen sauerstoff im player vom Enteren Raum
          (Default|SauerstoffImRaumSet (Variables|FürFirstRoom|GetAs%20BP%20Player) (Variables|Default|GetPlayerEnterRoom))
          ;[0.15 0.15 0.15 0.5] RoomcontainerÄnderrung
          (Variables|/Game/BP´s/Sauerstoff/BP_RoomContainer.BP_RoomContainer_C|SetIsPlayerInRoom (Variables|Default|GetPlayerEnterRoom) true)
          (Variables|/Game/BP´s/Sauerstoff/BP_RoomContainer.BP_RoomContainer_C|SetIsPlayerInRoom (Variables|Default|GetPlayerExitRoom) false)
          (if (Variables|Default|GetDebug)
            ;[0.15 0.15 0.15 0.5] debug
            (Development|PrintString (Utilities|String|Append "Print BP_SauerstoffRoomSwitsch --->  Exit : " (Variables|/Game/BP´s/Sauerstoff/BP_RoomContainer.BP_RoomContainer_C|GetMyRoomName (Variables|Default|GetPlayerExitRoom)) "                 Enter : " (Variables|/Game/BP´s/Sauerstoff/BP_RoomContainer.BP_RoomContainer_C|GetMyRoomName (Variables|Default|GetPlayerEnterRoom))) true true "(R=0.521266,G=1.000000,B=0.026755,A=1.000000)" 5.0))
          (Utilities|FlowControl|DoOnce false
            (:Completed
              (Default|PlayerEnterndRoom (Variables|Default|GetPlayerEnterRoom)))))))))

(fn ConstructionScript)