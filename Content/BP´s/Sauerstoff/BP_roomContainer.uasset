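; Room container Blueprint that tracks a room's oxygen (Sauerstoff) and drains it through registered holes while the player is inside.
; Unless the room is broken (KaputterRaum), PlayerEnterndRoom starts a looping timer; start rooms trigger it on BeginPlay and mark the player present.
; Each tick subtracts DecreaseAmount times the hole count from IRegestrateHole, clamping at zero and flagging the room empty.
; RaumNahmenRuecksendung returns the room name.
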(event Custom|PlayerEnterndRoom
  (if (not (Variables|Default|GetKaputterRaum))
    (Utilities|Time|SetTimerbyEvent (delegate Custom|DecreaseSauerstoff) (Variables|GamePlayEinstellungen|GetTriggerTime) true)))

(event Custom|DecreaseSauerstoff
  (bind _decreaseamount (Variables|GamePlayEinstellungen|GetDecreaseAmount))
  (bind _holeactorlist (Variables|Default|GetHoleActorList))
  (bind _returnvalue (Utilities|Array|Length _holeactorlist))
  (bind _returnvalue_2 (* _decreaseamount _returnvalue))
  (if (not (Variables|Default|GetKeinenSauerstoffMehrImRaum))
    (if (Variables|Default|GetIsPlayerInRoom)
      (bind _output_get (Variables|GamePlayEinstellungen|SetSauerstoffImRaum (- (Variables|GamePlayEinstellungen|GetSauerstoffImRaum) _returnvalue_2)))
      (if (Variables|Default|GetDebug)
        (Development|PrintString (Utilities|String|Append "Sauerstoff im raum ->   " (Variables|Default|GetMyRoomName) "    :   " (Utilities|String|ToString(Float) _output_get) "/         Wird abgezogen   :   " (Utilities|String|ToString(Float) _returnvalue_2)) true true "(R=0.515509,G=0.000000,B=1.000000,A=0.573913)" (- (Variables|GamePlayEinstellungen|GetTriggerTime) 0.1)))
      (if (<= (Variables|GamePlayEinstellungen|GetSauerstoffImRaum) 0.0)
        (Variables|GamePlayEinstellungen|SetSauerstoffImRaum 0.0)
        (Variables|Default|SetKeinenSauerstoffMehrImRaum true)
        (Development|PrintString "Sauerstoff 0" true true "(R=1.000000,G=0.819493,B=0.000000,A=1.000000)")))))

(event Custom|IregestrateHole
  (params (HoleActor :type BP%20Sauerstoff%20Lag%20Parent%20Object%20Reference)))

(event EventBeginPlay
  (Rendering|SetVisibility (Variables|Default|GetSphere) false false)
  (if (not (Variables|Default|GetKaputterRaum))
    (if (Variables|Default|GetRoomStart)
      (CallFunction|PlayerEnterndRoom)
      (Variables|Default|SetIsPlayerInRoom true))))

(event EventIRegestrateHole
  (params (HoleActor :type BP%20Sauerstoff%20Lag%20Parent%20Object%20Reference))
  ;[0.15 0.15 0.15 0.5] GibLoch Anzahl
  (bind _returnvalue (Utilities|Array|Add (Variables|Default|GetHoleActorList) HoleActor))
  (if (Variables|Default|GetDebug)
    (Development|PrintString (Utilities|String|Append (Utilities|String|ToString(Integer) _returnvalue) "  ----->  " (Utilities|GetDisplayName HoleActor)) true true "(R=0.000000,G=1.000000,B=0.088261,A=1.000000)")))

(fn ConstructionScript)

(fn RaumNahmenRuecksendung
  (return (Variables|Default|GetMyRoomName)))