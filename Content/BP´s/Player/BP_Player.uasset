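; First-person player character for a game with switchable gravity and oxygen survival, handling movement, interaction, pause and tutorial start.
; In zero gravity, a camera sphere trace places a grab actor that the player pulls toward, then release launches by charged push power.
; A looping timer drains oxygen by room level and hole repairs, updating MainUI and toggling a post-process when empty.
; Drift damping enables respawn when stranded, and timelines drive camera wobble.
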(event Custom|MoveInWorldDirection
  (params (Local%20Direction :type Vector))
  (bind _mainui (Variables|Default|GetMainUI))
  ;[0.15 0 0.1383 0.5] Player Steuerung
  ;;[0 0.01115 0.15 0.5] Mouvement
  (if (not (Variables|Default|GetMoveInputBlock))
    (if (not (Variables|Grap|GetIs%20Grapping))
      (if (not (Variables|Schwerkraft|GetSchwerkraftBoolFlip))
        (Pawn|Input|AddMovementInput (Math|Transform|TransformDirection (Math|Transform|MakeTransform "0, 0, 0" (Math|Rotator|MakeRotator 0.0 0.0 (.yaw (Transformation|GetWorldRotation (Variables|Default|GetCamera)))) "1.000000,1.000000,1.000000") Local%20Direction) 1.0 false)
        (Utilities|IsValid _mainui
          (:Is%20Valid
            (Default|AnyKeyWalkTotorial01 _mainui)))))))

(event Custom|Schwerkraft
  (params (Launch :type Boolean))
  ;[0.00405 0.15 0.002374 0.5] Umgebungseinflüsse
  ;;[0.08854 0.08854 0.08854 0.5] Schwerkraft An/Aus
  (bind _output_get (Variables|Schwerkraft|SetSchwerkraftBoolFlip (not (Variables|Schwerkraft|GetSchwerkraftBoolFlip))))
  (Variables|/Script/Engine.CharacterMovementComponent|SetGravityScale (Variables|Character|GetCharacterMovement) (Math|Float|SelectFloat 0.0 1.0 _output_get))
  (Variables|/Script/Engine.CharacterMovementComponent|SetGroundFriction (Variables|Character|GetCharacterMovement) (Math|Float|SelectFloat 0.0 8.0 _output_get))
  (Variables|/Script/Engine.CharacterMovementComponent|SetAirControl (Variables|Character|GetCharacterMovement) (Math|Float|SelectFloat 0.0 0.05 _output_get))
  (if Launch
    (Character|LaunchCharacter "0.000000,0.000000,75.000000" false false)
    (CallFunction|ZeroGravatystopscale)
    (Variables|Schwerkraft|SetPlayerSlowDownGravaty true)))

(event Custom|CamWigle
  (params (CamwigleInstantStop :type Boolean) (Stop :type Boolean))
  (bind _camera (Variables|Default|GetCamera))
  (bind _camera_2 (Variables|Default|GetCamera))
  (bind _returnvalue (Transformation|GetWorldRotation _camera_2))
  ;[0.15 0 0.09113 0.5] CamWigleAnimation
  (Variables|CamWigleAni|SetcamWigleInstantStop CamwigleInstantStop)
  (bind _output_get (Variables|CamWigleAni|SetCamIsWigle (not Stop)))
  (if _output_get
    (Utilities|FlowControl|Sequence
      (:then_0
        (bind _newtrack_0 (Timeline|WiggleAufbau PlayFromStart)
          (:Finished
            (if (Variables|CamWigleAni|GetCamIsWigle)
              (if (Variables|CamWigleAni|GetcamWigleInstantStop)
                (Variables|CamWigleAni|SetcamWigleInstantStop false)
                (Utilities|FlowControl|Delay 1.0)
                (Utilities|FlowControl|Sequence :!label _label
                  (:then_0
                    (bind _wiggle (Timeline|Wiggle Stop)
                      (:Update
                        (Utilities|FlowControl|Sequence
                          (:then_0
                            (Transformation|AddRelativeRotation (Variables|Default|GetCamera) (Math|Rotator|MakeRotator (* _wiggle (* _newtrack_0 (Variables|CamWigleAni|GetCamWigleStrongFloat))) 0.0 0.0) false false)
                            ;;[0.15 0.15 0.15 0.5] BugFix Cam rotate nach Rechts
                            (if (> (.roll _returnvalue) 1.1)
                              (Transformation|AddRelativeRotation (Variables|Default|GetCamera) (Math|Rotator|MakeRotator (* (.roll _returnvalue) -1.0) 0.0 0.0) false false)))
                          (:then_1
                            (Transformation|SetRelativeLocation (Variables|Default|GetCamera) (Math|Vector|MakeVector 0.0 0.0 (+ (* _wiggle (* _newtrack_0 (Variables|CamWigleAni|GetCamWigleStrongFloat))) (.z (Variables|CamWigleAni|GetcamPosttionSave)))) false false))))))
                  (:then_1
                    ;;[0.15 0.15 0.15 0.5] camreset
                    (Transformation|SetRelativeLocation (Variables|Default|GetCamera) (Variables|CamWigleAni|GetcamPosttionSave) false false)
                    (Transformation|AddRelativeRotation _camera (Math|Rotator|MakeRotator (* (.roll (Variables|/Script/Engine.SceneComponent|GetRelativeRotation _camera)) -1.0) 0.0 0.0) false false))))
              (else
                (goto _label))))))
      (:then_1
        (Timeline|Wiggle PlayFromStart)))
    (else
      (Utilities|FlowControl|Sequence
        (:then_1
          (Timeline|WiggleAufbau ReverseFromEnd))
        (:then_2)))))

(event Custom|AlarmAN/AUS
  (params (An :type Boolean))
  (bind _lichtleiste_zum_start_an_aus (Variables|Default|GetLichtleiste%20zum%20start%20an%20aus))
  ;[0.00405 0.15 0.002374 0.5] Umgebungseinflüsse
  (if An
    (Default|AlarmAn _lichtleiste_zum_start_an_aus)
    (else
      (Default|AlarmAus _lichtleiste_zum_start_an_aus))))

(event Custom|SauerstoffImRaumSet
  (params (Herkunft :type BP%20Room%20Container%20Object%20Reference))
  ;[0.08513 0.06576 0.526 0.5] Sauerstoff player/ UI
  ;;[0.15 0.15 0.15 0.5] Sauerstoff weiterleitung roomContainer --> UI trigger wenn player raum betritt
  ;;;[0.15 0.15 0.15 0.5] Aus BP_Sauerstorr_RoomSwitsch
  (Utilities|Time|SetTimerbyEvent (delegate Custom|Event%20Tick%20PlayerSauerstoff) (Variables|/Game/BP´s/Sauerstoff/BP_RoomContainer.BP_RoomContainer_C|GetTriggerTime Herkunft) true)
  (Default|EventBeginPLaySauerstoffinRoom (Variables|Default|GetMainUI) Herkunft self)
  ;;[0.15 0.15 0.15 0.5] HoleFixUpdate
  (Utilities|FlowControl|DelayUntilNextTick)
  (EventDispatchers|BindEventtoIsRoomDicht?-->Interfaces Herkunft (delegate Custom|klukshoifuzaou))
  ;;;[0.15 0.15 0.15 0.5] Abrufen von dichtigkeit ausm raum
  (Variables|SauerstoffEinstellungenTriggerTimeInJewaligenRaumEinstellbar|SetAllHolesFixed (Variables|/Game/BP´s/Sauerstoff/BP_RoomContainer.BP_RoomContainer_C|GetAreAllHolesFixed Herkunft)))

(event Custom|Event%20Tick%20PlayerSauerstoff
  ;[0.08513 0.06576 0.526 0.5] Sauerstoff player/ UI
  (if (not (Variables|SauerstoffEinstellungenTriggerTimeInJewaligenRaumEinstellbar|GetPlayersauerstoffAbzugStop))
    (bind _room_has___sauerstoff (Class|BPIHole|ImAktuellenRaumSind-->%(Message) (stale Custom|SauerstoffImRaumSet Herkunft)))
    ;;[0.15 0.15 0.15 0.5] Wert Aktualisiren
    (Variables|SauerstoffEinstellungenTriggerTimeInJewaligenRaumEinstellbar|SetPlayerSauetstoff (- (Variables|SauerstoffEinstellungenTriggerTimeInJewaligenRaumEinstellbar|GetPlayerSauetstoff) (* (Variables|SauerstoffEinstellungenTriggerTimeInJewaligenRaumEinstellbar|GetPlayeSauerstoffVerbrauch) (Math|Float|SelectFloat (- 1e+02 (Variables|/Game/BP´s/Sauerstoff/BP_RoomContainer.BP_RoomContainer_C|GetSauerstoff%20nach%20Holefix (stale Custom|SauerstoffImRaumSet Herkunft))) (- 1e+02 _room_has___sauerstoff) (Variables|SauerstoffEinstellungenTriggerTimeInJewaligenRaumEinstellbar|GetAllHolesFixed)))))
    ;;[0.15 0.15 0.15 0.5] %rechnung
    (Default|SauerstoffPlayerUI (Variables|Default|GetMainUI) (/ (* (Variables|SauerstoffEinstellungenTriggerTimeInJewaligenRaumEinstellbar|GetPlayerSauetstoff) 1e+02) (Variables|SauerstoffEinstellungenTriggerTimeInJewaligenRaumEinstellbar|GetPlayerSauerstoffBeginPlay)))
    (if (<= (Variables|SauerstoffEinstellungenTriggerTimeInJewaligenRaumEinstellbar|GetPlayerSauetstoff) 0.0)
      (Utilities|FlowControl|DoOnce false
        (:Completed
          (Variables|SauerstoffEinstellungenTriggerTimeInJewaligenRaumEinstellbar|SetSauerstoffauf0 true)
          (CallFunction|PostProcessOn/Off))))))

(event Custom|Interact
  (CallFunction|InteractFunction true))

(event Custom|PostProcess%20On/Off
  ;[0.15 0.15 0.15 0.5] PosrProcess
  (Utilities|FlowControl|FlipFlop
    (:A
      (Variables|PostProcess|SetWeight 1.0))
    (:B
      (Variables|PostProcess|SetWeight 0.0)))
  (bind _returnvalue (Rendering|Material|CreateDynamicMaterialInstance "/Game/Materials/PossProsses/MM_PP_01.MM_PP_01" "None" "None" :!class /Script/Engine.KismetMaterialLibrary))
  (Variables|/Script/Engine.CameraComponent|SetPostProcessSettings (Variables|Default|GetCamera) (Utilities|Struct|MakePostProcessSettings (Utilities|Struct|MakeWeightedBlendables (Utilities|Array|MakeArray (Utilities|Struct|MakeWeightedBlendable (Variables|PostProcess|GetWeight) _returnvalue))))))

(event Custom|klukshoifuzaou
  ;[0.08513 0.06576 0.526 0.5] Sauerstoff player/ UI
  ;;[0.15 0.15 0.15 0.5] HoleFixUpdate
  ;;;[0.15 0.15 0.15 0.5] Aktualisirung nach holefix
  ;;;[0.15 0.15 0.15 0.5] Abrufen von dichtigkeit ausm raum
  (Variables|SauerstoffEinstellungenTriggerTimeInJewaligenRaumEinstellbar|SetAllHolesFixed (Variables|/Game/BP´s/Sauerstoff/BP_RoomContainer.BP_RoomContainer_C|GetAreAllHolesFixed (stale Custom|SauerstoffImRaumSet Herkunft))))

(event Custom|ResetSauerstoff
  ;[0.08513 0.06576 0.526 0.5] Sauerstoff player/ UI
  ;;[0.15 0.15 0.15 0.5] Sauerstoff Wieder Auffüllen
  (Variables|CamWigleAni|SetAnimationstart%25 (Math|Float|SelectFloat 0.0 (/ (Variables|SauerstoffEinstellungenTriggerTimeInJewaligenRaumEinstellbar|GetPlayerSauetstoff) (/ (Variables|SauerstoffEinstellungenTriggerTimeInJewaligenRaumEinstellbar|GetPlayerSauerstoffBeginPlay) 1e+02)) (<= (/ (Variables|SauerstoffEinstellungenTriggerTimeInJewaligenRaumEinstellbar|GetPlayerSauetstoff) (/ (Variables|SauerstoffEinstellungenTriggerTimeInJewaligenRaumEinstellbar|GetPlayerSauerstoffBeginPlay) 1e+02)) 0.0)))
  (Variables|SauerstoffEinstellungenTriggerTimeInJewaligenRaumEinstellbar|SetPlayersauerstoffAbzugStop true)
  (bind _newtrack_0 (Timeline|Timeline PlayFromStart)
    (:Update
      (Variables|SauerstoffEinstellungenTriggerTimeInJewaligenRaumEinstellbar|SetPlayerSauetstoff (+ (* _newtrack_0 (* (/ (Variables|SauerstoffEinstellungenTriggerTimeInJewaligenRaumEinstellbar|GetPlayerSauerstoffBeginPlay) 1e+02) (- 1e+02 (Variables|CamWigleAni|GetAnimationstart%25)))) (* (/ (Variables|SauerstoffEinstellungenTriggerTimeInJewaligenRaumEinstellbar|GetPlayerSauerstoffBeginPlay) 1e+02) (Variables|CamWigleAni|GetAnimationstart%25))))
      ;;[0.15 0.15 0.15 0.5] %rechnung
      (Default|SauerstoffPlayerUI (Variables|Default|GetMainUI) (/ (* (Variables|SauerstoffEinstellungenTriggerTimeInJewaligenRaumEinstellbar|GetPlayerSauetstoff) 1e+02) (Variables|SauerstoffEinstellungenTriggerTimeInJewaligenRaumEinstellbar|GetPlayerSauerstoffBeginPlay)))
      (if (<= (Variables|SauerstoffEinstellungenTriggerTimeInJewaligenRaumEinstellbar|GetPlayerSauetstoff) 0.0)
        (Utilities|FlowControl|DoOnce false :!label _label
          (:Completed
            (Variables|SauerstoffEinstellungenTriggerTimeInJewaligenRaumEinstellbar|SetSauerstoffauf0 true)
            (CallFunction|PostProcessOn/Off)))))
    (:Finished
      (Variables|SauerstoffEinstellungenTriggerTimeInJewaligenRaumEinstellbar|SetPlayersauerstoffAbzugStop false)
      (if (Variables|SauerstoffEinstellungenTriggerTimeInJewaligenRaumEinstellbar|GetSauerstoffauf0)
        (CallFunction|PostProcessOn/Off)
        (Variables|SauerstoffEinstellungenTriggerTimeInJewaligenRaumEinstellbar|SetSauerstoffauf0 false)
        (goto _label Reset)))))

(event Custom|PlayerinputBlock_Event
  (Variables|Default|SetMoveInputBlock (not (Variables|Default|GetMoveInputBlock))))

(event Custom|SetNewRespawn
  (params (RespawnPoint :type Transform))
  ;[0.009944 0.15 0 0.5] Respawn
  (Variables|Default|SetRespawnPoint (Math|Transform|MakeTransform (.location RespawnPoint) (Transformation|GetActorRotation self) (.scale RespawnPoint))))

(event Custom|Festhalten
  (params (IsRelease :type Boolean))
  (bind _bp_grapactor (Variables|Grap|GetBP_GrapActor))
  ;[0 0.15 0.1461 0.5] Hand ranzehen und abstoßen
  ;;[0.15 0.15 0.15 0.5] bei schwerkraft aus
  (if (Variables|Schwerkraft|GetSchwerkraftBoolFlip)
    (if IsRelease
      (if (Variables|Grap|GetIs%20Grapping)
        (Variables|Grap|SetIs%20Grapping false)
        (Variables|Grap|SetGrapClose false)
        ;;[0.15 0.15 0.15 0.5] reset graphand
        (Rendering|SetVisibility (Variables|/Game/BP´s/Player/BP_GrapActor.BP_GrapActor_C|GetSphere (Variables|Grap|GetBP_GrapActor)) false false)
        (Transformation|SetWorldLocation (Variables|/Game/BP´s/Player/BP_GrapActor.BP_GrapActor_C|GetDefaultSceneRoot (Variables|Grap|GetBP_GrapActor)) "0, 0, 0" false true)
        ;;[0.15 0.1235 0 0.5] launch
        ;;;[0.15 0.15 0.15 0.5] Launch block
        (if (not (<= (Variables|Grap|GetPuschPower) 0.9))
          (if (Variables|Default|GetDebug)
            (Development|PrintString (Utilities|String|ToString(Vector) (* (Math|Vector|Normalize (- (Transformation|GetWorldLocation (Variables|Default|GetJumprichtung)) (Transformation|GetWorldLocation (Variables|Default|GetCamera)))) (* (Variables|Grap|GetPuschPower) (Variables|Grap|GetLaunchfloatMultiply))))))
          (Character|LaunchCharacter (* (Math|Vector|Normalize (- (Transformation|GetWorldLocation (Variables|Default|GetJumprichtung)) (Transformation|GetWorldLocation (Variables|Default|GetCamera)))) (* (Variables|Grap|GetPuschPower) (Variables|Grap|GetLaunchfloatMultiply))) false false)
          ;;[1 0 0 0.5] Umstellung wenn ich mit wiederstand innen und außen ohne wiederstand machen möchte
          (if true
            (Utilities|FlowControl|Delay 1.0)
            (Variables|Schwerkraft|SetPlayerSlowDownGravaty true))))
      (else
        (bind (_nothing_autput _handgrapposition) (CallFunction|InteractFunction false))
        (if (not _nothing_autput)
          ;;[0.15 0.15 0.15 0.5] Abspeichern von graplocation und setzen
          (bind _output_get (Variables|Grap|SetGraplocation _handgrapposition))
          (Transformation|SetWorldLocation (Variables|/Game/BP´s/Player/BP_GrapActor.BP_GrapActor_C|GetDefaultSceneRoot _bp_grapactor) _output_get false true)
          (Rendering|SetVisibility (Variables|/Game/BP´s/Player/BP_GrapActor.BP_GrapActor_C|GetSphere _bp_grapactor) true false)
          (Variables|Grap|SetIs%20Grapping true)
          ;;[0.15 0.15 0.15 0.5] be neu gappen wird punsch zurückgesetzt weil es je nach tich immer 1 zurück gesetzt wird
          (Variables|Grap|SetPuschPower 0.0)
          (Default|ResetPullStrenghtBar (Variables|Default|GetMainUI)))))))

(event Custom|ManuelBeginPlay
  (bind _startraum (Variables|Default|GetStartRaum))
  (bind _mainui (Variables|Default|GetMainUI))
  ;[0.15 0.15 0.15 0.5] aus BP_startcam
  (CallFunction|CreateWidget)
  (Default|CallManuelBeginPlayEventDispatscher)
  (EventDispatchers|AssignPlayerinputBlock (Variables|Default|GetMainUI) (delegate Custom|PlayerinputBlock_Event))
  ;[0.15 0.15 0.15 0.5] game start totorial
  (if (not (Variables|Default|GetDebug))
    (Utilities|FlowControl|Delay 1.0)
    (CallFunction|CamWigle true false)
    (Default|EventVisibilityTextboxFlip _mainui true)
    (Default|EventShowText _mainui 0 2 0.0)
    (Variables|Default|SetMoveInputBlock true)
    (Utilities|FlowControl|Delay 3.0)
    ;;[0.15 0.15 0.15 0.5] start Room Action
    (Utilities|FlowControl|DoOnce false
      (:Completed
        (Utilities|IsValid _startraum
          (:Is%20Valid
            (CallFunction|SauerstoffImRaumSet _startraum)
            (Default|EventRoomStart _startraum))
          (:Is%20Not%20Valid
            (Development|PrintString " Kein Start Raum" true true "(R=1.000000,G=0.001086,B=0.000032,A=1.000000)" 1e+01)))))))

(event Custom|PressRespawnButton
  ;[0.009944 0.15 0 0.5] Respawn
  (if (Variables|Default|GetCanPressRespawn)
    (Transformation|SetActorTransform (Variables|Default|GetRespawnPoint) false true)
    (Default|PlayerCanPressRespawnbuttonFlip (Variables|Default|GetMainUI))
    (Variables|Default|SetCanPressRespawn false)))

(event Custom|Event_EndGame
  ;[0.15 0.15 0.15 0.5] Aus BP_Ende
  (Variables|/Script/Engine.PlayerController|SetbShowMouseCursor (Game|GetPlayerController 0) true)
  (Development|ExecuteConsoleCommand "RestartLevel" 0))

(event Custom|Pause
  ;[0.15 0 0 0.5] Pause / Start (frag nicht)
  ;;[0.15 0.15 0.15 0.5] aus playercontroller
  (if (not (Variables|Default|GetPausePressBlock))
    (if (not (Variables|Default|GetGameHasPaused))
      (Variables|Default|SetGameHasPaused true)
      ;;[0.15 0.15 0.15 0.5] Für sauerstoffroomswitsch -> schon betretenen Room / Anfangsroom
      (Default|CallPressPause)
      (Widget|SetVisibility (Variables|Default|GetMainUI) "Hidden")
      (Variables|SauerstoffEinstellungenTriggerTimeInJewaligenRaumEinstellbar|SetPlayersauerstoffAbzugStop true))))

(event Custom|StartCam_HasPressPause
  ;[0.15 0 0 0.5] Pause / Start (frag nicht)
  ;;[0.15 0.15 0.15 0.5] Für sauerstoffroomswitsch -> schon betretenen Room / Anfangsroom
  (Default|CallPressPlay)
  (Variables|SauerstoffEinstellungenTriggerTimeInJewaligenRaumEinstellbar|SetPlayersauerstoffAbzugStop false))

(event Custom|Camcontroller
  (params (Action%20Valiue%20X :type Float%20%28double-precision%29) (Action%20Valiue%20Y :type Float%20%28double-precision%29))
  ;[0.15 0 0.1383 0.5] Player Steuerung
  ;;[0.15 0.15 0.15 0.5] CamRotation
  (Pawn|Input|AddControllerYawInput Action%20Valiue%20X)
  ;;;[0.15 0.15 0.15 0.5] bugfix
  (Transformation|AddRelativeRotation (Variables|Default|GetCamera) (Math|Rotator|MakeRotator 0.0 (* Action%20Valiue%20Y (Math|Float|SelectFloat 1.0 -1.0 (Variables|Default|GetIsUsingGamepad))) 0.0) false false))

(event Custom|Close
  ;[0 0.15 0.1461 0.5] Hand ranzehen und abstoßen
  ;;[0.15 0.15 0.15 0.5] von Grap Actor
  (Variables|Grap|SetGrapClose true)
  (Variables|/Script/Engine.MovementComponent|SetVelocity (Variables|Character|GetCharacterMovement) "0, 0, 0")
  ;;;[0.2604 0 0 0.5] bei schwerelosichkeit unnötig
  (Variables|/Script/Engine.CharacterMovementComponent|SetGravityScale (Variables|Character|GetCharacterMovement) 0.0))

(event Custom|Not%20close
  ;[0 0.15 0.1461 0.5] Hand ranzehen und abstoßen
  ;;[0.15 0.15 0.15 0.5] von Grap Actor
  (Variables|Grap|SetGrapClose false))

(event Custom|GrapjumpAufladung
  (params (Hold_Button :type Boolean))
  ;[0 0.15 0.1461 0.5] Hand ranzehen und abstoßen
  ;;[0.15 0.15 0.15 0.5] Push Power
  (if (Variables|Grap|GetIs%20Grapping)
    (if Hold_Button
      (if (not (>= (Variables|Grap|GetPuschPower) 1e+02))
        (bind _output_get (Variables|Grap|SetPuschPower (+ (Variables|Grap|GetPuschPower) 1.0)))
        (Default|PullStrenghtBar (Variables|Default|GetMainUI) _output_get)
        (Development|PrintString (Utilities|String|ToString(Float) _output_get) true true "(R=0.000000,G=0.660000,B=1.000000,A=1.000000)" 0.0)))))

(event Custom|PuschPowerBack_EventTick
  ;[0 0.15 0.1461 0.5] Hand ranzehen und abstoßen
  ;;[0.15 0.15 0.15 0.5] Push Power
  ;;;[0.15 0.15 0.15 0.5] kann raus genommen werden wenn blöd ist das bar nichst sovort weg ist
  (if (stale Custom|GrapjumpAufladung Hold_Button)
    (if (not (Variables|Grap|GetIs%20Grapping))
      (if (not (<= (Variables|Grap|GetPuschPower) 0.0)) :!label _label
        (Variables|Grap|SetPuschPower (- (Variables|Grap|GetPuschPower) 1.0))
        (Default|PullStrenghtBar (Variables|Default|GetMainUI) (stale Custom|GrapjumpAufladung _output_get))
        (Development|PrintString (Utilities|String|ToString(Float) (stale Custom|GrapjumpAufladung _output_get)) true true "(R=0.000000,G=0.660000,B=1.000000,A=1.000000)" 0.0)))
    (else
      (goto _label))))

(event Custom|zeroGravatystopscale
  (bind _camera (Variables|Default|GetCamera))
  (bind _returnvalue (Transformation|GetWorldLocation _camera))
  ;[0.00405 0.15 0.002374 0.5] Umgebungseinflüsse
  ;;[0.07812 0.07812 0.07812] schwebwiederstand
  (Utilities|FlowControl|Delay 0.2)
  (if (Variables|Schwerkraft|GetPlayerSlowDownGravaty)
    (bind _output_get (Variables|/Script/Engine.MovementComponent|SetVelocity (Variables|Character|GetCharacterMovement) (/ (Transformation|GetVelocity) 1.1)))
    (if true
      (Development|PrintString (Utilities|String|Append "Velosety" (Utilities|String|ToString(Vector) _output_get)) true true "(R=1.000000,G=0.866143,B=0.000000,A=1.000000)" 0.2))
    (if (Math|Boolean|ANDBoolean (<= (.X (Math|Vector|BreakVector _output_get)) 1.0) (<= (.Y (Math|Vector|BreakVector _output_get)) 1.0) (<= (.Z (Math|Vector|BreakVector _output_get)) 1.0) (>= (.X (Math|Vector|BreakVector _output_get)) -1.0) (>= (.Y (Math|Vector|BreakVector _output_get)) -1.0) (>= (.Z (Math|Vector|BreakVector _output_get)) -1.0))
      (Variables|/Script/Engine.MovementComponent|SetVelocity (Variables|Character|GetCharacterMovement) "0, 0, 0")
      (Variables|Schwerkraft|SetPlayerSlowDownGravaty false)
      ;;[0.15 0.15 0.15 0.5] Show ResetButton
      (bind _returnvalue_2 (Collision|MultiSphereTraceByChannel _returnvalue _returnvalue (Variables|Grap|GetMaxGrapRange) "TraceTypeQuery2" false 0 "None" true "(R=1.000000,G=0.000000,B=0.000000,A=1.000000)" "(R=0.000000,G=1.000000,B=0.000000,A=1.000000)" 1e+01))
      (if (not _returnvalue_2)
        (Variables|Default|SetCanPressRespawn true)
        (Development|PrintString "can press R")
        (Default|PlayerCanPressRespawnbuttonFlip (Variables|Default|GetMainUI))))))

(event Custom|Tick_PullOnHand
  ;[0 0.15 0.1461 0.5] Hand ranzehen und abstoßen
  ;;[0.15 0.15 0.15 0.5] ranzeihen an hand
  (if (Variables|Grap|GetIs%20Grapping)
    (if (not (Variables|Grap|GetGrapClose))
      (Character|LaunchCharacter (* (Math|Vector|Normalize (- (Variables|Grap|GetGraplocation) (Transformation|GetWorldLocation (Variables|Character|GetMesh)))) (Variables|Grap|GetMaxGrapRange)) false false))))

(event EventTick
  (params (DeltaSeconds :type Float%20%28single-precision%29))
  ;[0.3802 0 0 0.5] Event Tick
  (CallFunction|PuschPowerBackEventTick)
  (CallFunction|ZeroGravatystopscale)
  (CallFunction|TickPullonHand))

(event EventBeginPlay
  ;[0 0.3177 0.006203 0.5] Begin Play
  (Variables|SauerstoffEinstellungenTriggerTimeInJewaligenRaumEinstellbar|SetPlayerSauerstoffBeginPlay (Variables|SauerstoffEinstellungenTriggerTimeInJewaligenRaumEinstellbar|GetPlayerSauetstoff))
  (Variables|Default|SetGamestartPlayerGravityScale (Variables|/Script/Engine.CharacterMovementComponent|GetGravityScale (Variables|Character|GetCharacterMovement)))
  ;[0.15 0.15 0.15 0.5] CamWigleAnimation
  (Variables|CamWigleAni|SetcamPosttionSave (Variables|/Script/Engine.SceneComponent|GetRelativeLocation (Variables|Default|GetCamera))))

(event Input|KeyboardEvents|AnyKey
  (params (Key :type Key%20Structure :default "None"))
  (:Pressed
    (Variables|Default|SetIsUsingGamepad (Class|KismetInputLibrary|KeyIsGamepadKey Key))))

(event Input|KeyboardEvents|G
  (params (Key :type Key%20Structure :default "None"))
  ;[0.15 0.15 0.15 0.5] PosrProcess
  (:Pressed
    (Utilities|FlowControl|FlipFlop
      (:A
        (Variables|PostProcess|SetWeight 1.0))
      (:B
        (Variables|PostProcess|SetWeight 0.0)))
    (bind _returnvalue (Rendering|Material|CreateDynamicMaterialInstance "/Game/Materials/PossProsses/MM_PP_01.MM_PP_01" "None" "None" :!class /Script/Engine.KismetMaterialLibrary))
    (Variables|/Script/Engine.CameraComponent|SetPostProcessSettings (Variables|Default|GetCamera) (Utilities|Struct|MakePostProcessSettings (Utilities|Struct|MakeWeightedBlendables (Utilities|Array|MakeArray (Utilities|Struct|MakeWeightedBlendable (Variables|PostProcess|GetWeight) _returnvalue)))))))

(fn ConstructionScript)

(fn InteractFunction
  (params (CanInteract? :type Boolean))
  (bind _camera (Variables|Default|GetCamera))
  (bind _returnvalue (Transformation|GetWorldLocation _camera))
  ;[0.15 0.15 0.15 0.5] anvisiren von grapable wand
  (bind (_outhit _returnvalue_2) (Collision|SphereTraceByChannel _returnvalue (+ _returnvalue (* (Math|Vector|GetForwardVector _camera) (Variables|Grap|GetMaxGrapRange))) 1.0 "TraceTypeQuery2" false 0 "ForDuration" true "(R=1.000000,G=0.000000,B=0.000000,A=1.000000)" "(R=0.000000,G=1.000000,B=0.000000,A=1.000000)" 0.5))
  (if _returnvalue_2
    (if CanInteract?
      (if (Utilities|DoesObjectImplementInterface (.HitActor (Collision|BreakHitResult _outhit)) "/Game/BP´s/Player/BPI_Interact.BPI_Interact_C")
        ;[0.15 0.15 0.15 0.5] Hat Klebeband oder nicht
        (if (Utilities|DoesObjectImplementInterface (.HitActor (Collision|BreakHitResult _outhit)) "/Game/BP´s/Sauerstoff/BPI_Hole.BPI_Hole_C")
          (if (Variables|GenTeile|GetHasTape)
            (Class|BPIInteract|Interact(Message) (.HitActor (Collision|BreakHitResult _outhit)) self))
          (else
            (Class|BPIInteract|Interact(Message) (.HitActor (Collision|BreakHitResult _outhit)) self))))
      (else
        ;[0.15 0.1385 0.05391 0.5] positionssetzung füe GrabHand
        (return false (+ (.Location (Collision|BreakHitResult _outhit)) (* (Math|Vector|Normalize (- (.TraceStart (Collision|BreakHitResult _outhit)) (.Location (Collision|BreakHitResult _outhit)))) (Variables|Grap|Getsvere%28Hand%29%20von%20Wand%20Entfernt))))))
    (else
      (return true "0, 0, 0"))))

(fn CreateWidget
  (bind _returnvalue (UserInterface|CreateWidget "/Game/BP´s/UI/BPW_MainUI.BPW_MainUI_C" (Game|GetPlayerController 0)))
  (bind _output_get (Variables|Default|SetMainUI _returnvalue))
  (UserInterface|Viewport|AddtoPlayerScreen _output_get))