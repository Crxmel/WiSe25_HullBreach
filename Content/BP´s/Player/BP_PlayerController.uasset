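; Player controller that caches the possessed BP_Player and forwards player input to it.
; On BeginPlay it adds the IMC_Player Enhanced Input context; actions drive movement, camera, interaction, respawn and pause.
; Left-mouse press and release drive grabbing (Festhalten), while a held input drives grapple-jump charging (GrapjumpAufladung).
; Jump is gated by the pawn's gravity flag, a hard-coded 1 key calls Schwerkraft (gravity), and an alarm call is left unwired.
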(event Input|EnhancedActionEvents|EnhancedInputActionIA_PlayerMove
  (params (ActionValue :type Vector%202D%20Structure) (ElapsedSeconds :type Float%20%28double-precision%29) (TriggeredSeconds :type Float%20%28double-precision%29) (InputAction :type Input%20Action%20Object%20Reference :default "/Game/Imputs/PlayerInputs/IA_PlayerMove.IA_PlayerMove"))
  ;[0.002854 0.004849 0.15 0.5] movement
  (Default|MoveinWorldDirection (Variables|Default|GetPosess%20Character) (Math|Vector|MakeVector (.x ActionValue) (.y ActionValue) 0.0)))

(event Input|EnhancedActionEvents|EnhancedInputActionIA_PlayerCamRotation
  (params (ActionValue :type Vector%202D%20Structure) (ElapsedSeconds :type Float%20%28double-precision%29) (TriggeredSeconds :type Float%20%28double-precision%29) (InputAction :type Input%20Action%20Object%20Reference :default "/Game/Imputs/PlayerInputs/IA_PlayerCamRotation.IA_PlayerCamRotation"))
  ;[0.15 0.128 0 0.5] Cam Rotation
  (Default|Camcontroller (Variables|Default|GetPosess%20Character) (.x ActionValue) (.y ActionValue)))

(event Input|EnhancedActionEvents|EnhancedInputActionIA_Jump
  (params (ActionValue :type Boolean) (ElapsedSeconds :type Float%20%28double-precision%29) (TriggeredSeconds :type Float%20%28double-precision%29) (InputAction :type Input%20Action%20Object%20Reference :default "/Game/Imputs/PlayerInputs/IA_Jump.IA_Jump"))
  (if (not (Variables|/Game/BP´s/Player/BP_Player.BP_Player_C|GetSchwerkraftBoolFlip (Variables|Default|GetPosess%20Character)))
    (Character|Jump (Variables|Default|GetPosess%20Character))))

(event Input|EnhancedActionEvents|EnhancedInputActionIA_Pause
  (params (ActionValue :type Boolean) (ElapsedSeconds :type Float%20%28double-precision%29) (TriggeredSeconds :type Float%20%28double-precision%29) (InputAction :type Input%20Action%20Object%20Reference :default "/Game/Imputs/PlayerInputs/IA_Pause.IA_Pause"))
  (Default|Pause (Variables|Default|GetPosess%20Character)))

(event Input|EnhancedActionEvents|EnhancedInputActionIA_LMB
  (params (ActionValue :type Boolean) (ElapsedSeconds :type Float%20%28double-precision%29) (TriggeredSeconds :type Float%20%28double-precision%29) (InputAction :type Input%20Action%20Object%20Reference :default "/Game/Imputs/PlayerInputs/IA_LMB.IA_LMB"))
  (:Started
    (Variables|Default|SetGrapPressedReleaseFlip false)
    (Default|Festhalten (Variables|Default|GetPosess%20Character) (Variables|Default|GetGrapPressedReleaseFlip) :!label _label))
  (:Completed
    (Variables|Default|SetGrapPressedReleaseFlip true)
    (goto _label)))

(event Input|EnhancedActionEvents|EnhancedInputActionIA_LodePullStrenght
  (params (ActionValue :type Boolean) (ElapsedSeconds :type Float%20%28double-precision%29) (TriggeredSeconds :type Float%20%28double-precision%29) (InputAction :type Input%20Action%20Object%20Reference :default "/Game/Imputs/PlayerInputs/IA_LodePullStrenght.IA_LodePullStrenght"))
  (:Triggered
    (Default|GrapjumpAufladung (Variables|Default|GetPosess%20Character) (Variables|Default|GetHold_Button) :!label _label))
  (:Started
    (Variables|Default|SetHold_Button true))
  (:Completed
    (Variables|Default|SetHold_Button false)
    (goto _label)))

(event Input|EnhancedActionEvents|EnhancedInputActionIA_Interact
  (params (ActionValue :type Boolean) (ElapsedSeconds :type Float%20%28double-precision%29) (TriggeredSeconds :type Float%20%28double-precision%29) (InputAction :type Input%20Action%20Object%20Reference :default "/Game/Imputs/PlayerInputs/IA_Interact.IA_Interact"))
  (Default|Interact (Variables|Default|GetPosess%20Character)))

(event Input|EnhancedActionEvents|EnhancedInputActionIA_Respawn
  (params (ActionValue :type Boolean) (ElapsedSeconds :type Float%20%28double-precision%29) (TriggeredSeconds :type Float%20%28double-precision%29) (InputAction :type Input%20Action%20Object%20Reference :default "/Game/Imputs/PlayerInputs/IA_Respawn.IA_Respawn"))
  (Default|PressRespawnButton (Variables|Default|GetPosess%20Character)))

(event EventBeginPlay
  (Input|AddMappingContext (PlayerController|LocalPlayerSubsystems|GetEnhancedInputLocalPlayerSubsystem) "/Game/Imputs/IMC_Player.IMC_Player" 0 "(bIgnoreAllPressedKeysUntilRelease=True,bForceImmediately=False,bNotifyUserSettings=False)"))

(event EventPossess
  (params (PossessedPawn :type Pawn%20Object%20Reference))
  (bind _asbp_player (Utilities|Casting|CastToBP_Player PossessedPawn))
  (Variables|Default|SetPosess%20Character _asbp_player))

(event Input|KeyboardEvents|1
  (params (Key :type Key%20Structure :default "None"))
  (:Pressed
    (Default|Schwerkraft (Variables|Default|GetPosess%20Character) false)))

(fn ConstructionScript)