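; Light strip actor whose five point lights dim one after another, chained to neighboring BP_lichtleiste strips.
; Each strip finds and caches its neighbor by overlapping its left or right sphere, chosen by LightwayR.
; A strip flagged as light start re-triggers the chain from Tick through a Delay, and each strip relays Lichttrigger, guarded against same-frame re-entry.
; Each trigger lowers intensity by Steps, with later lights starting as the previous one drops below staggered thresholds.
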(event Custom|Lichttrigger
  (if (CallFunction|TimeHasPassedSinceLastHits)
    (Variables|Default|SetLastHitTime (Utilities|Time|GetGameTimeinSeconds))
    (Utilities|FlowControl|Sequence
      (:then_0
        (CallFunction|NextLightSave))
      (:then_1
        (Utilities|FlowControl|DoOnce false
          (:Completed
            (bind _output_get (Variables|einzelneLichtspeicher|SetLight_1 (Variables|Default|Getlightsave)))
            (bind _output_get_2 (Variables|einzelneLichtspeicher|SetLight_2 _output_get))
            (bind _output_get_3 (Variables|einzelneLichtspeicher|SetLight_3 _output_get_2))
            (bind _output_get_4 (Variables|einzelneLichtspeicher|SetLight_4 _output_get_3))
            (Variables|einzelneLichtspeicher|SetLight_5 _output_get_4))))
      (:then_2
        (if (not (<= (Variables|einzelneLichtspeicher|GetLight_1) 0.0))
          (bind _output_get_5 (Variables|einzelneLichtspeicher|SetLight_1 (- (Variables|einzelneLichtspeicher|GetLight_1) (Variables|Animationgeschwindickkeit|GetSteps))))
          (Rendering|Components|Light|SetIntensity (Variables|Default|GetPointLight) _output_get_5)
          (Development|PrintString (Utilities|String|ToString(Float) _output_get_5) true true "(R=0.000000,G=0.660000,B=1.000000,A=1.000000)" (Variables|Animationgeschwindickkeit|GetAnimationDuration))))
      (:then_3
        (if (and (< (Variables|einzelneLichtspeicher|GetLight_1) (* (/ (Variables|Default|Getlightsave) (Variables|Animationgeschwindickkeit|GetÜbergangsHärte)) 4.0)) (not (<= (Variables|einzelneLichtspeicher|GetLight_2) 0.0)))
          (bind _output_get_6 (Variables|einzelneLichtspeicher|SetLight_2 (- (Variables|einzelneLichtspeicher|GetLight_2) (Variables|Animationgeschwindickkeit|GetSteps))))
          (Rendering|Components|Light|SetIntensity (Variables|Default|GetPointLight1) _output_get_6)))
      (:then_4
        (if (and (< (Variables|einzelneLichtspeicher|GetLight_2) (* (/ (Variables|Default|Getlightsave) (Variables|Animationgeschwindickkeit|GetÜbergangsHärte)) 3.0)) (not (<= (Variables|einzelneLichtspeicher|GetLight_3) 0.0)))
          (bind _output_get_7 (Variables|einzelneLichtspeicher|SetLight_3 (- (Variables|einzelneLichtspeicher|GetLight_3) (Variables|Animationgeschwindickkeit|GetSteps))))
          (Rendering|Components|Light|SetIntensity (Variables|Default|GetPointLight2) _output_get_7)))
      (:then_5
        (if (and (< (Variables|einzelneLichtspeicher|GetLight_3) (* (/ (Variables|Default|Getlightsave) (Variables|Animationgeschwindickkeit|GetÜbergangsHärte)) 2.0)) (not (<= (Variables|einzelneLichtspeicher|GetLight_4) 0.0)))
          (bind _output_get_8 (Variables|einzelneLichtspeicher|SetLight_4 (- (Variables|einzelneLichtspeicher|GetLight_4) (Variables|Animationgeschwindickkeit|GetSteps))))
          (Rendering|Components|Light|SetIntensity (Variables|Default|GetPointLight3) _output_get_8)))
      (:then_6
        (if (< (Variables|einzelneLichtspeicher|GetLight_4) (* (/ (Variables|Default|Getlightsave) (Variables|Animationgeschwindickkeit|GetÜbergangsHärte)) 1.0))
          (bind _output_get_9 (Variables|einzelneLichtspeicher|SetLight_5 (- (Variables|einzelneLichtspeicher|GetLight_5) (Variables|Animationgeschwindickkeit|GetSteps))))
          (Rendering|Components|Light|SetIntensity (Variables|Default|GetPointLight4) _output_get_9))))))

(event EventBeginPlay
  (bind _output_get (Variables|Default|SetLightIntensity (Variables|/Script/Engine.LightComponentBase|GetIntensity (Variables|Default|GetPointLight))))
  (Variables|Default|Setlightsave _output_get)
  (CallFunction|NextLightSave))

(event EventTick
  (params (DeltaSeconds :type Float%20%28single-precision%29))
  (if (Variables|Default|GetligthStart)
    (Utilities|FlowControl|Delay (Variables|Animationgeschwindickkeit|GetAnimationDuration))
    (if (Variables|Default|GetStart)
      (CallFunction|NextLightSave))))

(fn ConstructionScript)

(fn NextLightSave
  (Utilities|IsValid (Variables|Default|GetNextLight)
    (:Is%20Valid
      (CallFunction|Lichttrigger (Variables|Default|GetNextLight)))
    (:Is%20Not%20Valid
      (bind _newlocalvar1 (CallFunction|Test))
      (Variables|Default|SetNextLight _newlocalvar1))))

(fn LightAnimation
  (params (NewParam :type Point%20Light%20Component%20Object%20Reference) (Steps :type Float%20%28double-precision%29))
  (Utilities|FlowControl|Sequence
    (:then_0
      (Utilities|FlowControl|DoOnce false
        (:Completed
          (bind _output_get (LocalVariables|SetLight_1 (Variables|Default|Getlightsave)))
          (LocalVariables|SetLight_2 _output_get))))
    (:then_1
      (bind _output_get_2 (LocalVariables|SetLight_1 (- (LocalVariables|GetLight_1) Steps)))
      (Rendering|Components|Light|SetIntensity (Variables|Default|GetPointLight) _output_get_2)
      (Development|PrintString (Utilities|String|ToString(Float) _output_get_2) true true "(R=0.000000,G=0.660000,B=1.000000,A=1.000000)" (Variables|Animationgeschwindickkeit|GetAnimationDuration)))
    (:then_2
      (if (< (LocalVariables|GetLight_1) (* (/ (Variables|Default|Getlightsave) 5.0) 4.0))
        (bind _output_get_3 (LocalVariables|SetLight_2 (- (LocalVariables|GetLight_2) Steps)))
        (Rendering|Components|Light|SetIntensity (Variables|Default|GetPointLight1) _output_get_3)))))

(fn TimeHasPassedSinceLastHits
  (return (> (Utilities|Time|GetGameTimeinSeconds) (Variables|Default|GetLastHitTime))))

(fn Test
  (bind _self self)
  (bind _animationduration (Variables|Animationgeschwindickkeit|GetAnimationDuration))
  (bind _nextlight (Variables|Default|GetNextLight))
  (bind _returnvalue (Utilities|GetObjectName _self))
  (bind _returnvalue_2 (- _animationduration 0.1))
  (bind (_outactors _returnvalue_3) (Collision|SphereOverlapActors (Transformation|GetWorldLocation (select (Variables|Default|GetLightway_R) (Variables|Default|GetR_Sphere) (Variables|Default|GetL_Sphere))) (Math|Float|SelectFloat (Components|Sphere|GetScaledSphereRadius (Variables|Default|GetL_Sphere)) (Components|Sphere|GetScaledSphereRadius (Variables|Default|GetR_Sphere)) (Variables|Default|GetLightway_R)) (Utilities|Array|MakeArray "ObjectTypeQuery1" "ObjectTypeQuery2" "ObjectTypeQuery4" "ObjectTypeQuery3") "BP_lichtleiste_C"))
  (if _returnvalue_3
    (for _array_element _outactors
      (bind _asbp_lichtleiste (Utilities|Casting|CastToBP_lichtleiste _array_element)
        (:then
          (LocalVariables|SetNewLocalVar _asbp_lichtleiste)
          (Development|PrintString (Utilities|String|Append _returnvalue ": cast") true true "(R=0.000000,G=0.660000,B=1.000000,A=1.000000)" _returnvalue_2))
        (:CastFailed
          (Utilities|IsValid _nextlight
            (:Is%20Valid
              (LocalVariables|SetNewLocalVar _nextlight)
              (Development|PrintString (Utilities|String|Append _returnvalue ": cast falled") true true "(R=0.000000,G=0.660000,B=1.000000,A=1.000000)" _returnvalue_2))
            (:Is%20Not%20Valid
              (Development|PrintString (Utilities|String|Append _returnvalue " : dont set Next Light or Start Light") true true "(R=1.000000,G=0.000000,B=0.025861,A=1.000000)" 1e+01)
              (bind _output_get (LocalVariables|SetNewLocalVar 0))
              (return _output_get)))))
      (Variables|Default|SetStart true)
      (CallFunction|Lichttrigger (LocalVariables|GetNewLocalVar))
      (return (LocalVariables|GetNewLocalVar)))
    (else
      (return 0))))