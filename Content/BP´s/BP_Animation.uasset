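; BP_Animation is a trigger actor that plays a scripted room-destruction sequence when BP_Player leaves its overlap area.
; It pauses oxygen drain, locks movement and starts the alarm, then after timed delays shakes the camera, calls the player's gravity function, unlocks movement and destroys the linked room.
; A timeline then rotates and wobbles a referenced mesh, stopping the camera shake and resuming oxygen drain when finished.
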(event Collision|EventActorEndOverlap
  (params (OtherActor :type Actor%20Object%20Reference))
  (bind _asbp_player (Utilities|Casting|CastToBP_Player OtherActor))
  (Variables|Default|SetAs%20BP%20Player _asbp_player)
  ;[0.15 0.15 0.15 0.5] sauerstoffabzug stop
  (Variables|/Game/BP´s/Player/BP_Player.BP_Player_C|SetPlayersauerstoffAbzugStop (Variables|Default|GetAs%20BP%20Player) true)
  (Variables|/Game/BP´s/Player/BP_Player.BP_Player_C|SetMoveInputBlock (Variables|Default|GetAs%20BP%20Player) true)
  (Default|AlarmAN/AUS (Variables|Default|GetAs%20BP%20Player) true)
  (Utilities|FlowControl|Delay (Variables|Default|GetAlarmAN-->CamWigleDelay))
  (Default|CamWigle (Variables|Default|GetAs%20BP%20Player) false false)
  (Utilities|FlowControl|Delay (Variables|Default|GetActionDelay))
  (Default|Schwerkraft (Variables|Default|GetAs%20BP%20Player) true)
  (Variables|/Game/BP´s/Player/BP_Player.BP_Player_C|SetMoveInputBlock (Variables|Default|GetAs%20BP%20Player) false)
  (Default|RoomGetDestroyed (Variables|Default|GetDestroyedRoom))
  (bind (_direction _rotationsanimation _wigleanimation) (Timeline|Timeline PlayFromStart)
    (:Update
      (Transformation|SetWorldRotation (Variables|/Script/Engine.StaticMeshActor|GetStaticMeshComponent (Variables|Default|GetRotationMesh)) (Math|Rotator|MakeRotator 0.0 (* _wigleanimation 1.0) (* _rotationsanimation (Variables|Default|GetMeshRotation))) false false))
    (:Finished
      (Default|CamWigle (Variables|Default|GetAs%20BP%20Player) false true)
      ;[0.15 0.15 0.15 0.5] sauerstoffabzug weiter
      (Variables|/Game/BP´s/Player/BP_Player.BP_Player_C|SetPlayersauerstoffAbzugStop (Variables|Default|GetAs%20BP%20Player) false))))

(fn ConstructionScript)