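; Parent Blueprint for a room-destruction event with rope-based repair, driven by a rotating, wiggling mesh.
; When the player first leaves its overlap, it triggers alarm, camera wiggle and gravity calls, destroys the linked room and plays the animation timeline.
; RepareSeil counts placed ropes; at eight it repairs the room, calls the RoomIsRepared hook and reverses the timeline.
; Timeline completion sets oxygen drain, flips rope input blocking and can start tutorial two.
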(event Custom|RepareSeil
  (params (IsPlace :type Boolean))
  (bind _as_bp_player (Variables|Default|GetAs%20BP%20Player))
  (bind _as_bp_player_2 (Variables|Default|GetAs%20BP%20Player))
  (bind _mainui (Variables|/Game/BP´s/Player/BP_Player.BP_Player_C|GetMainUI _as_bp_player_2))
  (if IsPlace
    (Variables|Default|SetSeilePlatzirt (+ (Variables|Default|GetSeilePlatzirt) 1))
    (else
      (Variables|Default|SetSeilePlatzirt (- (Variables|Default|GetSeilePlatzirt) 1))))
  ;[0.15 0.15 0.15 0.5] sind alle seile platzirt
  (if (== (Variables|Default|GetSeilePlatzirt) 8)
    (Default|CallReparaturseilInputBlockFlip)
    (Default|RoomGetRepared (Variables|Default|GetDestroyedRoom))
    (CallFunction|RoomIsRepared)
    (bind (_direction _rotationsanimation _wigleanimation) (Timeline|Timeline ReverseFromEnd)
      (:Update
        (Transformation|SetWorldRotation (Variables|/Script/Engine.StaticMeshActor|GetStaticMeshComponent (Variables|Default|GetRotationMesh)) (Math|Rotator|MakeRotator 0.0 (* _wigleanimation (select (== (Variables|Default|GetSeilePlatzirt) 8) 0.0 1.0)) (* _rotationsanimation (Variables|Default|GetMeshRotation))) false false))
      (:Finished
        (Utilities|IsValid (Variables|Default|GetAs%20BP%20Player)
          (:Is%20Valid
            (Utilities|FlowControl|Sequence
              (:then_0
                (if (== (Variables|Default|GetSeilePlatzirt) 8)
                  ;[0.15 0.15 0.15 0.5] sauerstoffabzug weiter
                  (Variables|/Game/BP´s/Player/BP_Player.BP_Player_C|SetPlayersauerstoffAbzugStop (Variables|Default|GetAs%20BP%20Player) true)
                  (Default|CallReparaturseilInputBlockFlip)
                  (else
                    (Default|CamWigle _as_bp_player false true)
                    ;[0.15 0.15 0.15 0.5] sauerstoffabzug weiter
                    (Variables|/Game/BP´s/Player/BP_Player.BP_Player_C|SetPlayersauerstoffAbzugStop _as_bp_player false)
                    (Default|CallReparaturseilInputBlockFlip))))
              (:then_1
                ;[0.15 0.1196 0 0.5] Totorial 2 start nach 5ten Text
                (if (== (Variables|/Game/BP´s/UI/BPW_MainUI.BPW_MainUI_C|Get%20First%20Show%20Text%20Number _mainui) 5)
                  (Default|VisualTotorialStart02 _mainui))))))))
    (else
      (Development|PrintString (Utilities|String|ToString(Integer) (Variables|Default|GetSeilePlatzirt))))))

(event Custom|DestroyRoomEvent
  (bind _as_bp_player (Variables|Default|GetAs%20BP%20Player))
  (bind _as_bp_player_2 (Variables|Default|GetAs%20BP%20Player))
  (bind _mainui (Variables|/Game/BP´s/Player/BP_Player.BP_Player_C|GetMainUI _as_bp_player_2))
  (Utilities|FlowControl|DoOnce false
    (:Completed
      (bind (_direction _rotationsanimation _wigleanimation) (Timeline|Timeline PlayFromStart)
        (:Update
          (Transformation|SetWorldRotation (Variables|/Script/Engine.StaticMeshActor|GetStaticMeshComponent (Variables|Default|GetRotationMesh)) (Math|Rotator|MakeRotator 0.0 (* _wigleanimation (select (== (Variables|Default|GetSeilePlatzirt) 8) 0.0 1.0)) (* _rotationsanimation (Variables|Default|GetMeshRotation))) false false))
        (:Finished
          (Utilities|IsValid (Variables|Default|GetAs%20BP%20Player)
            (:Is%20Valid
              (Utilities|FlowControl|Sequence
                (:then_0
                  (if (== (Variables|Default|GetSeilePlatzirt) 8)
                    ;[0.15 0.15 0.15 0.5] sauerstoffabzug weiter
                    (Variables|/Game/BP´s/Player/BP_Player.BP_Player_C|SetPlayersauerstoffAbzugStop (Variables|Default|GetAs%20BP%20Player) true)
                    (Default|CallReparaturseilInputBlockFlip)
                    (else
                      (Default|CamWigle _as_bp_player false true)
                      ;[0.15 0.15 0.15 0.5] sauerstoffabzug weiter
                      (Variables|/Game/BP´s/Player/BP_Player.BP_Player_C|SetPlayersauerstoffAbzugStop _as_bp_player false)
                      (Default|CallReparaturseilInputBlockFlip))))
                (:then_1
                  ;[0.15 0.1196 0 0.5] Totorial 2 start nach 5ten Text
                  (if (== (Variables|/Game/BP´s/UI/BPW_MainUI.BPW_MainUI_C|Get%20First%20Show%20Text%20Number _mainui) 5)
                    (Default|VisualTotorialStart02 _mainui)))))))))))

(event Custom|RoomIsRepared)

(event Collision|EventActorEndOverlap
  (params (OtherActor :type Actor%20Object%20Reference))
  (Utilities|FlowControl|DoOnce false
    (:Completed
      (bind _asbp_player (Utilities|Casting|CastToBP_Player OtherActor))
      (Variables|Default|SetAs%20BP%20Player _asbp_player)
      ;[0.15 0.15 0.15 0.5] sauerstoffabzug stop
      (Variables|/Game/BP´s/Player/BP_Player.BP_Player_C|SetPlayersauerstoffAbzugStop (Variables|Default|GetAs%20BP%20Player) true)
      (Default|AlarmAN/AUS (Variables|Default|GetAs%20BP%20Player) true)
      (Utilities|FlowControl|Delay (Variables|Default|GetAlarmAN-->CamWigleDelay))
      (Default|CamWigle (Variables|Default|GetAs%20BP%20Player) false false)
      (Utilities|FlowControl|Delay (Variables|Default|GetActionDelay))
      (Default|Schwerkraft (Variables|Default|GetAs%20BP%20Player) true)
      (Variables|/Game/BP´s/Player/BP_Player.BP_Player_C|SetMoveInputBlock (Variables|Default|GetAs%20BP%20Player) false)
      (Default|RoomGetDestroyed (Variables|Default|GetDestroyedRoom))
      (bind (_direction _rotationsanimation _wigleanimation) (Timeline|Timeline PlayFromStart)
        (:Update
          (Transformation|SetWorldRotation (Variables|/Script/Engine.StaticMeshActor|GetStaticMeshComponent (Variables|Default|GetRotationMesh)) (Math|Rotator|MakeRotator 0.0 (* _wigleanimation (select (== (Variables|Default|GetSeilePlatzirt) 8) 0.0 1.0)) (* _rotationsanimation (Variables|Default|GetMeshRotation))) false false))
        (:Finished
          (Utilities|IsValid (Variables|Default|GetAs%20BP%20Player)
            (:Is%20Valid
              (Utilities|FlowControl|Sequence
                (:then_0
                  (if (== (Variables|Default|GetSeilePlatzirt) 8)
                    ;[0.15 0.15 0.15 0.5] sauerstoffabzug weiter
                    (Variables|/Game/BP´s/Player/BP_Player.BP_Player_C|SetPlayersauerstoffAbzugStop (Variables|Default|GetAs%20BP%20Player) true)
                    (Default|CallReparaturseilInputBlockFlip)
                    (else
                      (Default|CamWigle (Variables|Default|GetAs%20BP%20Player) false true)
                      ;[0.15 0.15 0.15 0.5] sauerstoffabzug weiter
                      (Variables|/Game/BP´s/Player/BP_Player.BP_Player_C|SetPlayersauerstoffAbzugStop (Variables|Default|GetAs%20BP%20Player) false)
                      (Default|CallReparaturseilInputBlockFlip))))
                (:then_1
                  ;[0.15 0.1196 0 0.5] Totorial 2 start nach 5ten Text
                  (if (== (Variables|/Game/BP´s/UI/BPW_MainUI.BPW_MainUI_C|Get%20First%20Show%20Text%20Number (Variables|/Game/BP´s/Player/BP_Player.BP_Player_C|GetMainUI (Variables|Default|GetAs%20BP%20Player))) 5)
                    (Default|VisualTotorialStart02 (Variables|/Game/BP´s/Player/BP_Player.BP_Player_C|GetMainUI (Variables|Default|GetAs%20BP%20Player)))))))))))))

(fn ConstructionScript)

(fn TriggerDialog)