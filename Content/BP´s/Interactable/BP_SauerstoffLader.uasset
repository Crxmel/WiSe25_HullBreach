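; BP_SauerstoffLader is an interactable oxygen charger that resets the player's oxygen (Sauerstoff) when used.
; Its Interact event calls the parent implementation, then ResetSauerstoff on the interacting player.
; A DoOnce then sets the player's FirstInteractWithSauerstoffinteract flag, only on the first use of that charger instance.
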(event EventBeginPlay
  (|CallParentFunction) ; This node is disabled and will not be called.\nDrag off pins to build functionality.
)

(event Collision|EventActorBeginOverlap
  (params (OtherActor :type Actor%20Object%20Reference))
  (|CallParentFunction OtherActor) ; This node is disabled and will not be called.\nDrag off pins to build functionality.
)

(event EventTick
  (params (DeltaSeconds :type Float%20%28single-precision%29))
  (|CallParentFunction DeltaSeconds) ; This node is disabled and will not be called.\nDrag off pins to build functionality.
)

(event EventInteract
  (params (Player :type BP%20Player%20Object%20Reference))
  (|CallParentFunction Player)
  (Default|ResetSauerstoff Player)
  (Utilities|FlowControl|DoOnce false
    (:Completed
      (Variables|/Game/BP´s/Player/BP_Player.BP_Player_C|SetFirstInteractWithSauerstoffinteract Player true))))

(fn ConstructionScript
  (|CallParentFunction))