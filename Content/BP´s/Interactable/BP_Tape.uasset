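; BP_Tape is an interactable tape pickup that grants the tape to the player who interacts with it.
; On Interact, unless InteractBlock is set, it runs the parent interaction, sets the player's HasTape flag and hides its Cylinder mesh.
; It then flips InteractBlock through a separate event, so the pickup works only once and the actor stays in the level, hidden.
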(event Custom|InteractBlockFlipEvent
  (Variables|Default|SetInteractBlock (not (Variables|Default|GetInteractBlock))))

(event EventInteract
  (params (Player :type BP%20Player%20Object%20Reference))
  (if (not (Variables|Default|GetInteractBlock))
    (|CallParentFunction Player)
    (Variables|/Game/BP´s/Player/BP_Player.BP_Player_C|SetHasTape (Variables|Default|GetPlayer) true)
    (Rendering|SetVisibility (Variables|Default|GetCylinder) false false)
    (CallFunction|InteractBlockFlipEvent)))

(fn ConstructionScript
  (|CallParentFunction))