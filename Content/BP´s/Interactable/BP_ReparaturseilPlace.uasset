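; BP_ReparaturseilPlace is an interactable spot where the player places or retrieves a repair rope.
; Interact moves a rope between the player's counter and the spot, toggling the Cube's visibility and SeliIsPlace state.
; Each change is passed to the linked ZuReparireneAnimation object through RepareSeil.
; That object's dispatcher flips an input-block flag, but the check on it is disconnected, so interaction is never blocked here.
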(event Custom|ReparaturseilInputBlockFlip_Event
  (bind _output_get (Variables|Default|SetInputIsBlock (not (Variables|Default|GetInputIsBlock)))))

(event EventInteract
  (params (Player :type BP%20Player%20Object%20Reference))
  (|CallParentFunction Player)
  (if (== (Variables|/Game/BP´s/Player/BP_Player.BP_Player_C|GetReperaturseilcount (Variables|Default|GetPlayer)) 0)
    (if (Variables|Default|GetSeliIsPlace)
      (Variables|/Game/BP´s/Player/BP_Player.BP_Player_C|SetReperaturseilcount (Variables|Default|GetPlayer) (+ (Variables|/Game/BP´s/Player/BP_Player.BP_Player_C|GetReperaturseilcount (Variables|Default|GetPlayer)) 1) :!label _label)
      (Rendering|SetVisibility (Variables|Default|GetCube) false false)
      (Variables|Default|SetSeliIsPlace false)
      (Default|RepareSeil (Variables|Default|GetZuReparireneAnimation) (Variables|Default|GetSeliIsPlace) :!label _label_2))
    (elif (Variables|Default|GetSeliIsPlace)
      (goto _label)
      (else
        (Variables|/Game/BP´s/Player/BP_Player.BP_Player_C|SetReperaturseilcount (Variables|Default|GetPlayer) (- (Variables|/Game/BP´s/Player/BP_Player.BP_Player_C|GetReperaturseilcount (Variables|Default|GetPlayer)) 1))
        (Rendering|SetVisibility (Variables|Default|GetCube) true false)
        (Variables|Default|SetSeliIsPlace true)
        (goto _label_2)))))

(event EventBeginPlay
  (|CallParentFunction)
  (EventDispatchers|AssignReparaturseilInputBlockFlip (Variables|Default|GetZuReparireneAnimation) (delegate Custom|ReparaturseilInputBlockFlip_Event)))

(fn ConstructionScript
  (|CallParentFunction))