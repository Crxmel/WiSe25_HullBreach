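; BP_Startcam is a possessable menu camera that hosts the start, pause and end-game screen.
; On begin play, player pause or game end, it creates BPW_Menu, blends the view to itself, takes possession and swaps character input for puzzle input.
; Game end also hides the button bar and flags credits to play.
; Leaving the screen returns view, possession and input to the player, running its manual begin-play first time, otherwise restoring its UI.
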(event Custom|Start/PauseScreenOff
  (bind _player (Variables|Default|GetPlayer))
  (bind _mainui (Variables|/Game/BP´s/Player/BP_Player.BP_Player_C|GetMainUI _player))
  ;[0.15 0.15 0.15 0.5] für rausauerstoff abzug weiter
  (Default|StartCamHasPressPause (Variables|Default|GetPlayer))
  (Input|RemoveMappingContext (PlayerController|LocalPlayerSubsystems|GetEnhancedInputLocalPlayerSubsystem (Game|GetPlayerController 0)) (Variables|Default|GetPuzzleMappingContext) "(bIgnoreAllPressedKeysUntilRelease=True,bForceImmediately=False,bNotifyUserSettings=False)")
  (Game|Player|SetViewTargetwithBlend (Game|GetPlayerController 0) (Variables|Default|GetPlayer) (Variables|Default|GetSmoothProssessDuration) "VTBlend_Linear" 0.0 false)
  (Utilities|FlowControl|Delay (Variables|Default|GetSmoothProssessDuration))
  (Pawn|Possess (Game|GetPlayerController 0) (Variables|Default|GetPlayer))
  (Input|AddMappingContext (PlayerController|LocalPlayerSubsystems|GetEnhancedInputLocalPlayerSubsystem (Game|GetPlayerController 0)) (Variables|Default|GetCharakterMappingContext) 0 "(bIgnoreAllPressedKeysUntilRelease=True,bForceImmediately=False,bNotifyUserSettings=False)")
  (if (Variables|Default|GetFirstDialogHasPlayed)
    (Default|CreateWidget _player)
    (Widget|SetVisibility _mainui "Visible")
    (Variables|/Game/BP´s/UI/BPW_MainUI.BPW_MainUI_C|SetGameIsPaused _mainui false)
    (Default|PLay _player)
    (else
      (Default|ManuelBeginPlay (Variables|Default|GetPlayer))
      (Variables|Default|SetFirstDialogHasPlayed true))))

(event Custom|Start/PauseScreenOn
  (bind _returnvalue (UserInterface|CreateWidget "/Game/BP´s/UI/BPW_Menu.BPW_Menu_C" (Game|GetPlayerController 0)))
  (bind _output_get (Variables|Default|SetMenu _returnvalue))
  (UserInterface|Viewport|AddtoPlayerScreen _output_get)
  (Input|RemoveMappingContext (PlayerController|LocalPlayerSubsystems|GetEnhancedInputLocalPlayerSubsystem (Game|GetPlayerController 0)) (Variables|Default|GetCharakterMappingContext) "(bIgnoreAllPressedKeysUntilRelease=True,bForceImmediately=False,bNotifyUserSettings=False)")
  (Game|Player|SetViewTargetwithBlend (Game|GetPlayerController 0) self (Variables|Default|GetSmoothProssessDuration) "VTBlend_Linear" 0.0 false)
  (Utilities|FlowControl|Delay (Variables|Default|GetSmoothProssessDuration))
  (Pawn|Possess (Game|GetPlayerController 0) self)
  (Input|AddMappingContext (PlayerController|LocalPlayerSubsystems|GetEnhancedInputLocalPlayerSubsystem (Game|GetPlayerController 0)) (Variables|Default|GetPuzzleMappingContext) 0 "(bIgnoreAllPressedKeysUntilRelease=True,bForceImmediately=False,bNotifyUserSettings=False)")
  (Default|SavePlayer (Variables|Default|GetMenu) self))

(event Custom|CustomEvent
  (Utilities|FlowControl|Sequence
    (:then_0
      (bind _returnvalue (UserInterface|CreateWidget "/Game/BP´s/UI/BPW_Menu.BPW_Menu_C" (Game|GetPlayerController 0)))
      (bind _output_get (Variables|Default|SetMenu _returnvalue))
      (UserInterface|Viewport|AddtoPlayerScreen _output_get)
      (Input|RemoveMappingContext (PlayerController|LocalPlayerSubsystems|GetEnhancedInputLocalPlayerSubsystem (Game|GetPlayerController 0)) (Variables|Default|GetCharakterMappingContext) "(bIgnoreAllPressedKeysUntilRelease=True,bForceImmediately=False,bNotifyUserSettings=False)")
      (Game|Player|SetViewTargetwithBlend (Game|GetPlayerController 0) self (Variables|Default|GetSmoothProssessDuration) "VTBlend_Linear" 0.0 false)
      (Utilities|FlowControl|Delay (Variables|Default|GetSmoothProssessDuration))
      (Pawn|Possess (Game|GetPlayerController 0) self)
      (Input|AddMappingContext (PlayerController|LocalPlayerSubsystems|GetEnhancedInputLocalPlayerSubsystem (Game|GetPlayerController 0)) (Variables|Default|GetPuzzleMappingContext) 0 "(bIgnoreAllPressedKeysUntilRelease=True,bForceImmediately=False,bNotifyUserSettings=False)")
      (Default|SavePlayer (Variables|Default|GetMenu) self))
    (:then_1
      (Widget|SetVisibility (Variables|/Game/BP´s/UI/BPW_Menu.BPW_Menu_C|GetButtonsleiste (Variables|Default|GetMenu)) "Hidden")
      (Variables|/Game/BP´s/UI/BPW_Menu.BPW_Menu_C|SetCreditsPlay (Variables|Default|GetMenu) true))))

(event EventBeginPlay
  (bind _player (Variables|Default|GetPlayer))
  (EventDispatchers|BindEventtoEndGame _player (delegate Custom|CustomEvent))
  (EventDispatchers|BindEventtoPressPause _player (delegate Custom|Start/PauseScreenOn))
  (bind _returnvalue (UserInterface|CreateWidget "/Game/BP´s/UI/BPW_Menu.BPW_Menu_C" (Game|GetPlayerController 0)))
  (bind _output_get (Variables|Default|SetMenu _returnvalue))
  (UserInterface|Viewport|AddtoPlayerScreen _output_get)
  (Input|RemoveMappingContext (PlayerController|LocalPlayerSubsystems|GetEnhancedInputLocalPlayerSubsystem (Game|GetPlayerController 0)) (Variables|Default|GetCharakterMappingContext) "(bIgnoreAllPressedKeysUntilRelease=True,bForceImmediately=False,bNotifyUserSettings=False)")
  (Game|Player|SetViewTargetwithBlend (Game|GetPlayerController 0) self (Variables|Default|GetSmoothProssessDuration) "VTBlend_Linear" 0.0 false)
  (Utilities|FlowControl|Delay (Variables|Default|GetSmoothProssessDuration))
  (Pawn|Possess (Game|GetPlayerController 0) self)
  (Input|AddMappingContext (PlayerController|LocalPlayerSubsystems|GetEnhancedInputLocalPlayerSubsystem (Game|GetPlayerController 0)) (Variables|Default|GetPuzzleMappingContext) 0 "(bIgnoreAllPressedKeysUntilRelease=True,bForceImmediately=False,bNotifyUserSettings=False)")
  (Default|SavePlayer (Variables|Default|GetMenu) self))

(fn ConstructionScript)