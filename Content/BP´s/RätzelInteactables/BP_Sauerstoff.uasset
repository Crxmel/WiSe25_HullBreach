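; Possessable oxygen generator puzzle that switches on once it has both player-collected filter parts and the toolbox.
; Possessing it moves a carried toolbox onto the generator (clearable by pickup), then shows dialogue, naming missing items when only some are present.
; Text advances drive camera and rotation timelines, reversed on the third box to return to the character.
; After the completion text, it sets GenIstAn and notifies all BPI_Hole actors.
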(event Custom|WerkzeugAufgehoben_Event
  ;[0.15 0.15 0.15 0.5] Possess text
  ;;[0.15 0.15 0.15 0.5] Wenn werkzeug am gen aufgehoben wurde wird bool umgesetzt das er kein werkzeug hier hat
  (Variables|Default|SetGenHasWerkzeug_2 false))

(event EventNextTextTriggerEvent
  ;[0.15 0.15 0.15 0.5] Animation trigger + schwerkraft/strom bei textcount
  (if (Variables|Default|GetIsPossessed)
    (if (not (Variables|Default|GetGenIstAn))
      (|CallParentFunction)
      (Utilities|FlowControl|Sequence
        (:then_0
          (Variables|Default|SetFirs%20text%20has%20read true)
          (Variables|Default|Settextbos%20has%20seen (+ (Variables|Default|Gettextbos%20has%20seen) 1))
          ;;[0.15 0.15 0.15 0.5] close or open by triggert TextBoxCount
          (if (== (Variables|Default|Gettextbos%20has%20seen) 1)
            ;;[0.15 0.15 0.15 0.5] Animation
            (Utilities|FlowControl|Sequence
              (:then_0
                (Utilities|FlowControl|Delay 0.1)
                (bind _newtrack_0 (Timeline|Timeline_0 PlayFromStart)
                  (:Update
                    (Transformation|AddRelativeLocation (Variables|Default|GetCamera_sauer) (Math|Vector|MakeVector (* _newtrack_0 (select (== (Variables|Default|Gettextbos%20has%20seen) 3) -1.0 1.0)) 0.0 0.0) false false))))
              (:then_1
                (bind _newtrack_0_2 (Timeline|Timeline PlayFromStart)
                  (:Update
                    (Transformation|SetRelativeRotation (Variables|Default|GetRotationsPoint) (Math|Rotator|MakeRotator 0.0 (* _newtrack_0_2 45.0) 0.0) false false))
                  (:Finished
                    (if (== (Variables|Default|Gettextbos%20has%20seen) 3)
                      (CallFunction|ReturntoCharacter)
                      (Variables|Default|SetIsPossessed false))))))
            (elif (== (Variables|Default|Gettextbos%20has%20seen) 3)
              (Utilities|FlowControl|Sequence
                (:then_0
                  (Timeline|Timeline_0 ReverseFromEnd))
                (:then_1
                  (Utilities|FlowControl|Delay 0.1)
                  (Timeline|Timeline ReverseFromEnd))))))
        (:then_1
          (if (Variables|Default|GetPlayerReadFinishText)
            (if (== (Variables|Default|Gettextbos%20has%20seen) 3)
              (Variables|Default|SetGenIstAn true)
              (bind _outactors (Actor|GetAllActorswithInterface "/Game/BP´s/Sauerstoff/BPI_Hole.BPI_Hole_C"))
              (for _array_element _outactors
                (Class|BPIHole|SauerstoffgenIson(Message) _array_element)))))))))

(event EventReturntoCharacter
  ;[0.15 0.15 0.15 0.5] Animation trigger + schwerkraft/strom bei textcount
  ;;[0.15 0.15 0.15 0.5] Reset by exit
  (|CallParentFunction)
  (Variables|Default|Settextbos%20has%20seen 0))

(event EventEventGetPossessed
  (bind _player (Variables|Default|GetPlayer))
  (bind _player_2 (Variables|Default|GetPlayer))
  (bind _player_3 (Variables|Default|GetPlayer))
  (bind _felende_inteactable_text_ende (Variables|Default|GetFelende%20inteactable%20text%20ende))
  (bind _visiblewerkzeug (Variables|Default|GetVisibleWerkzeug))
  (bind _sauerstoffteil_filter_02 (Variables|/Game/BP´s/Player/BP_Player.BP_Player_C|GetSauerstoffTeil_Filter_02 _player))
  ;[0.15 0.15 0.15 0.5] Possess text
  (Variables|Default|SetIsPossessed true)
  (if (Variables|Default|GetGenIstAn)
    (CallFunction|UITrigger 10 10)
    (else
      (|CallParentFunction)
      ;;[0.15 0.15 0.15 0.5] Wenn werkzeug am gen aufgehoben wurde wird bool umgesetzt das er kein werkzeug hier hat
      (EventDispatchers|AssignWerkzeugAufgehoben (Variables|Default|GetVisibleWerkzeug) (delegate Custom|WerkzeugAufgehoben_Event))
      (Utilities|FlowControl|Sequence
        (:then_0
          (Utilities|FlowControl|DelayUntilNextTick)
          ;;[0.15 0.15 0.15 0.5] Hat noch nix text
          (if (Math|Boolean|ORBoolean (Variables|/Game/BP´s/Player/BP_Player.BP_Player_C|GetSauerstoffTeil_Filter_01 _player_2) (Variables|/Game/BP´s/Player/BP_Player.BP_Player_C|GetSauerstoffTeil_Filter_02 _player_2) (Variables|Default|GetGenHasWerkzeug_2))
            ;;[0.15 0.15 0.15 0.5] hat alle
            (if (Math|Boolean|ANDBoolean (Variables|/Game/BP´s/Player/BP_Player.BP_Player_C|GetSauerstoffTeil_Filter_01 _player_3) (Variables|/Game/BP´s/Player/BP_Player.BP_Player_C|GetSauerstoffTeil_Filter_02 _player_3) (Variables|Default|GetGenHasWerkzeug_2))
              ;;[0.15 0.15 0.15 0.5] finish text
              (Variables|Default|SetPlayerReadFinishText true)
              (Default|SetNewTextEvent (Variables|/Game/BP´s/Player/BP_Player.BP_Player_C|GetMainUI (Variables|Default|GetPlayer)) 11 (Variables|Default|GetDontHasAllPicesText))
              (Utilities|FlowControl|DelayUntilNextTick)
              (Default|SetNewTextEvent (Variables|/Game/BP´s/Player/BP_Player.BP_Player_C|GetMainUI (Variables|Default|GetPlayer)) 13 (Variables|Default|GetHasAllPicesText_02))
              (CallFunction|UITrigger 11 13)
              (else
                ;;[0.15 0.15 0.15 0.5] Custom text
                (Default|SetNewTextEvent (Variables|/Game/BP´s/Player/BP_Player.BP_Player_C|GetMainUI (Variables|Default|GetPlayer)) 11 (Variables|Default|GetDontHasAllPicesText))
                (Utilities|FlowControl|DelayUntilNextTick)
                (Default|SetNewTextEvent (Variables|/Game/BP´s/Player/BP_Player.BP_Player_C|GetMainUI (Variables|Default|GetPlayer)) 13 (Utilities|Text|ToText(String) (Utilities|String|Append "Mir fehlt noch " (select (Variables|/Game/BP´s/Player/BP_Player.BP_Player_C|GetSauerstoffTeil_Filter_01 _player) (select _sauerstoffteil_filter_02 (select (Variables|Default|GetGenHasWerkzeug_2) _felende_inteactable_text_ende (Utilities|String|Append "Das Werkzeug " _felende_inteactable_text_ende)) (Utilities|String|Append (select (Variables|Default|GetGenHasWerkzeug_2) "was zum filtern  " "was zum filtern und  ") (select (Variables|Default|GetGenHasWerkzeug_2) _felende_inteactable_text_ende (Utilities|String|Append "Das Werkzeug " _felende_inteactable_text_ende)))) (Utilities|String|Append (select (and (Variables|Default|GetGenHasWerkzeug_2) _sauerstoffteil_filter_02) "was zum filtern " "was zum filtern und  ") (select _sauerstoffteil_filter_02 (select (Variables|Default|GetGenHasWerkzeug_2) _felende_inteactable_text_ende (Utilities|String|Append "Das Werkzeug " _felende_inteactable_text_ende)) (Utilities|String|Append (select (Variables|Default|GetGenHasWerkzeug_2) "was zum filtern  " "was zum filtern und  ") (select (Variables|Default|GetGenHasWerkzeug_2) _felende_inteactable_text_ende (Utilities|String|Append "Das Werkzeug " _felende_inteactable_text_ende)))))))))
                (CallFunction|UITrigger 11 13)))
            (else
              (CallFunction|UITrigger 11 13))))
        (:then_1
          ;;[0.15 0.15 0.15 0.5] Wenn wekreug in player wird der an gen ab gelegt und im player umgestellt
          (if (Variables|/Game/BP´s/Player/BP_Player.BP_Player_C|GetWerkzeugKasten (Variables|Default|GetPlayer))
            (Variables|Default|SetGenHasWerkzeug_2 true)
            (Variables|/Game/BP´s/Player/BP_Player.BP_Player_C|SetWerkzeugKasten (Variables|Default|GetPlayer) false)
            (Rendering|SetVisibility (Variables|/Game/BP´s/Interactable/BP_Interact_Parent.BP_Interact_Parent_C|GetDefaultSceneRoot _visiblewerkzeug) true true)
            (Default|InteractBlockFlipEvent _visiblewerkzeug)))))))

(fn ConstructionScript
  (|CallParentFunction))

(fn UITrigger
  (params (%20First%20Show%20Text%20Number :type Integer) (Last%20Show%20Text%20Number :type Integer))
  (bind _player (Variables|Default|GetPlayer))
  (bind _mainui (Variables|/Game/BP´s/Player/BP_Player.BP_Player_C|GetMainUI _player))
  (Default|EventVisibilityTextboxFlip _mainui true)
  (Default|EventShowText _mainui %20First%20Show%20Text%20Number Last%20Show%20Text%20Number (Variables|Default|GetUIPressNextButtonDelay)))