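; BP_Gen is a possessable generator puzzle that the player repairs with a hose, fuse and toolbox.
; On possession it builds German dialogue naming missing parts and takes a carried toolbox, which can be picked up again.
; Dialogue advances play timelines that swing two pivots and slide the camera, reversing on the third step to release possession.
; Once the completion text is read, it switches gravity and alarm states and notifies EndeCollider.
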(event Custom|WerkzeugAufgehoben_Event
  ;[0.15 0.15 0.15 0.5] Possess text
  ;;[0.15 0.15 0.15 0.5] Wenn werkzeug am gen aufgehoben wurde wird bool umgesetzt das er kein werkzeug hier hat
  (Variables|Default|SetGenHasWerkzeug false))

(event EventNextTextTriggerEvent
  (bind _player (Variables|Default|GetPlayer))
  ;[0.15 0.15 0.15 0.5] Animation trigger + schwerkraft/strom bei textcount
  (if (Variables|Default|GetIsPossessed)
    (if (not (Variables|Default|GetGenIstAn))
      (|CallParentFunction)
      (Utilities|FlowControl|Sequence
        (:then_0
          (Variables|Default|SetFirs%20text%20has%20read true)
          (Variables|Default|Settextbos%20has%20seen (+ (Variables|Default|Gettextbos%20has%20seen) 1))
          ;;[0.15 0.15 0.15 0.5] close or open by triggert TextBoxCount
          (if (== (Variables|Default|Gettextbos%20has%20seen) 1)
            ;;[0.15 0.15 0.15 0.5] Animation
            (Utilities|FlowControl|Sequence
              (:then_0
                (Utilities|FlowControl|Delay 0.1)
                (bind _newtrack_0 (Timeline|Timeline_0 PlayFromStart)
                  (:Update
                    (Transformation|AddRelativeLocation (Variables|Default|GetCamera_gen) (Math|Vector|MakeVector (* _newtrack_0 (select (== (Variables|Default|Gettextbos%20has%20seen) 3) -1.0 1.0)) 0.0 0.0) false false))))
              (:then_1
                (bind _newtrack_0_2 (Timeline|Timeline PlayFromStart)
                  (:Update
                    (Transformation|SetRelativeRotation (Variables|Default|GetRotationsPoint_L) (Math|Rotator|MakeRotator 0.0 0.0 (* _newtrack_0_2 45.0)) false false)
                    (Transformation|SetRelativeRotation (Variables|Default|GetRotationsPoint_R) (Math|Rotator|MakeRotator 0.0 0.0 (* (* _newtrack_0_2 45.0) -1.0)) false false))
                  (:Finished
                    (if (== (Variables|Default|Gettextbos%20has%20seen) 3)
                      (CallFunction|ReturntoCharacter)
                      (Variables|Default|SetIsPossessed false))))))
            (elif (== (Variables|Default|Gettextbos%20has%20seen) 3)
              (Utilities|FlowControl|Sequence
                (:then_0
                  (Timeline|Timeline_0 ReverseFromEnd))
                (:then_1
                  (Utilities|FlowControl|Delay 0.1)
                  (Timeline|Timeline ReverseFromEnd))))))
        (:then_1
          ;;[0.15 0.15 0.15 0.5] wenn lezter text gelesen wird und duich ist wird strom und schwerkraft an gemacht
          (if (Variables|Default|GetPlayerReadFinishText)
            (if (== (Variables|Default|Gettextbos%20has%20seen) 3)
              (Default|Schwerkraft _player false)
              (Default|AlarmAN/AUS _player false)
              (Variables|Default|SetGenIstAn true)
              (Default|BigThingRepared (Variables|Default|GetEndeCollider) true false false false))))))))

(event EventReturntoCharacter
  ;[0.15 0.15 0.15 0.5] Animation trigger + schwerkraft/strom bei textcount
  ;;[0.15 0.15 0.15 0.5] Reset by exit
  (|CallParentFunction)
  (Variables|Default|Settextbos%20has%20seen 0))

(event EventEventGetPossessed
  (bind _player (Variables|Default|GetPlayer))
  (bind _felende_inteactable_text_ende (Variables|Default|GetFelende%20inteactable%20text%20ende))
  (bind _player_2 (Variables|Default|GetPlayer))
  (bind _player_3 (Variables|Default|GetPlayer))
  (bind _visiblewerkzeug (Variables|Default|GetVisibleWerkzeug))
  (bind _genteil_sicherrung (Variables|/Game/BP´s/Player/BP_Player.BP_Player_C|GetGenTeil_Sicherrung _player_3))
  ;[0.15 0.15 0.15 0.5] Possess text
  (Variables|Default|SetIsPossessed true)
  (if (Variables|Default|GetGenIstAn)
    (CallFunction|UITrigger 10 10)
    (else
      (|CallParentFunction)
      ;;[0.15 0.15 0.15 0.5] Wenn werkzeug am gen aufgehoben wurde wird bool umgesetzt das er kein werkzeug hier hat
      (EventDispatchers|AssignWerkzeugAufgehoben (Variables|Default|GetVisibleWerkzeug) (delegate Custom|WerkzeugAufgehoben_Event))
      (Utilities|FlowControl|Sequence
        (:then_0
          (Utilities|FlowControl|DelayUntilNextTick)
          ;;[0.15 0.15 0.15 0.5] Hat noch nix text
          (if (Math|Boolean|ORBoolean (Variables|/Game/BP´s/Player/BP_Player.BP_Player_C|GetGenTeil_Schlauch _player) (Variables|/Game/BP´s/Player/BP_Player.BP_Player_C|GetGenTeil_Sicherrung _player) (Variables|Default|GetGenHasWerkzeug))
            ;;[0.15 0.15 0.15 0.5] hat alle
            (if (Math|Boolean|ANDBoolean (Variables|/Game/BP´s/Player/BP_Player.BP_Player_C|GetGenTeil_Schlauch _player_2) (Variables|/Game/BP´s/Player/BP_Player.BP_Player_C|GetGenTeil_Sicherrung _player_2) (Variables|Default|GetGenHasWerkzeug))
              ;;[0.15 0.15 0.15 0.5] finish text
              (Development|PrintString "finish text" true true "(R=0.000000,G=1.000000,B=0.079728,A=1.000000)")
              (Variables|Default|SetPlayerReadFinishText true)
              (Default|SetNewTextEvent (Variables|/Game/BP´s/Player/BP_Player.BP_Player_C|GetMainUI (Variables|Default|GetPlayer)) 7 (Variables|Default|GetDontHasAllPicesText))
              (Utilities|FlowControl|DelayUntilNextTick)
              (Default|SetNewTextEvent (Variables|/Game/BP´s/Player/BP_Player.BP_Player_C|GetMainUI (Variables|Default|GetPlayer)) 9 (Variables|Default|GetHasAllPicesText_02))
              (CallFunction|UITrigger 7 9)
              (else
                ;;[0.15 0.15 0.15 0.5] Custom text
                (Default|SetNewTextEvent (Variables|/Game/BP´s/Player/BP_Player.BP_Player_C|GetMainUI (Variables|Default|GetPlayer)) 7 (Variables|Default|GetDontHasAllPicesText))
                (Utilities|FlowControl|DelayUntilNextTick)
                (Default|SetNewTextEvent (Variables|/Game/BP´s/Player/BP_Player.BP_Player_C|GetMainUI (Variables|Default|GetPlayer)) 9 (Utilities|Text|ToText(String) (Utilities|String|Append "Mir fehlt noch " (select (Variables|/Game/BP´s/Player/BP_Player.BP_Player_C|GetGenTeil_Schlauch _player_3) (select _genteil_sicherrung (select (Variables|Default|GetGenHasWerkzeug) _felende_inteactable_text_ende (Utilities|String|Append "Das Werkzeug " _felende_inteactable_text_ende)) (Utilities|String|Append (select (Variables|Default|GetGenHasWerkzeug) "Die Sicherrung " "Die Sicherrung und ") (select (Variables|Default|GetGenHasWerkzeug) _felende_inteactable_text_ende (Utilities|String|Append "Das Werkzeug " _felende_inteactable_text_ende)))) (Utilities|String|Append (select (and (Variables|Default|GetGenHasWerkzeug) _genteil_sicherrung) "ein schlauch" "ein Schlauch und ") (select _genteil_sicherrung (select (Variables|Default|GetGenHasWerkzeug) _felende_inteactable_text_ende (Utilities|String|Append "Das Werkzeug " _felende_inteactable_text_ende)) (Utilities|String|Append (select (Variables|Default|GetGenHasWerkzeug) "Die Sicherrung " "Die Sicherrung und ") (select (Variables|Default|GetGenHasWerkzeug) _felende_inteactable_text_ende (Utilities|String|Append "Das Werkzeug " _felende_inteactable_text_ende)))))))))
                (CallFunction|UITrigger 7 9)))
            (else
              (Development|PrintString "First text version" true true "(R=0.000000,G=0.660000,B=1.000000,A=0.426087)" 5.0)
              (CallFunction|UITrigger 7 9))))
        (:then_1
          ;;[0.15 0.15 0.15 0.5] Wenn wekreug in player wird der an gen ab gelegt und im player umgestellt
          (if (Variables|/Game/BP´s/Player/BP_Player.BP_Player_C|GetWerkzeugKasten (Variables|Default|GetPlayer))
            (Variables|Default|SetGenHasWerkzeug true)
            (Variables|/Game/BP´s/Player/BP_Player.BP_Player_C|SetWerkzeugKasten (Variables|Default|GetPlayer) false)
            (Rendering|SetVisibility (Variables|/Game/BP´s/Interactable/BP_Interact_Parent.BP_Interact_Parent_C|GetDefaultSceneRoot _visiblewerkzeug) true true)
            (Default|InteractBlockFlipEvent _visiblewerkzeug)))))))

(fn ConstructionScript
  (|CallParentFunction))

(fn UITrigger
  (params (%20First%20Show%20Text%20Number :type Integer) (Last%20Show%20Text%20Number :type Integer))
  (bind _player (Variables|Default|GetPlayer))
  (bind _mainui (Variables|/Game/BP´s/Player/BP_Player.BP_Player_C|GetMainUI _player))
  (Default|EventVisibilityTextboxFlip _mainui true)
  (Default|EventShowText _mainui %20First%20Show%20Text%20Number Last%20Show%20Text%20Number (Variables|Default|GetUIPressNextButtonDelay)))