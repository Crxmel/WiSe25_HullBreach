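; Parent pawn for puzzle interactables that the player takes control of on interaction and leaves with the puzzle escape input.
; Interact hands MainUI an empty next-text event, blends the view to the puzzle, then possesses it and swaps character input mapping for puzzle mapping.
; Escape reverses this after moving the character to the puzzle camera's yaw and floor point, found by a downward trace plus capsule half-height, with debug output left on.
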(event Custom|Event_GetPossessed
  (Input|RemoveMappingContext (PlayerController|LocalPlayerSubsystems|GetEnhancedInputLocalPlayerSubsystem (Game|GetPlayerController 0)) (Variables|Default|GetCharakterMappingContext) "(bIgnoreAllPressedKeysUntilRelease=True,bForceImmediately=False,bNotifyUserSettings=False)")
  (Game|Player|SetViewTargetwithBlend (Game|GetPlayerController 0) self (Variables|Default|GetSmoothProssessDuration) "VTBlend_Linear" 0.0 false)
  (Utilities|FlowControl|Delay (Variables|Default|GetSmoothProssessDuration))
  (Pawn|Possess (Game|GetPlayerController 0) self)
  (Input|AddMappingContext (PlayerController|LocalPlayerSubsystems|GetEnhancedInputLocalPlayerSubsystem (Game|GetPlayerController 0)) (Variables|Default|GetPuzzleMappingContext) 0 "(bIgnoreAllPressedKeysUntilRelease=True,bForceImmediately=False,bNotifyUserSettings=False)"))

(event Custom|ReturnToCharacter
  (CallFunction|PositionPlayerCharacter)
  (Input|RemoveMappingContext (PlayerController|LocalPlayerSubsystems|GetEnhancedInputLocalPlayerSubsystem (Game|GetPlayerController 0)) (Variables|Default|GetPuzzleMappingContext) "(bIgnoreAllPressedKeysUntilRelease=True,bForceImmediately=False,bNotifyUserSettings=False)")
  (Game|Player|SetViewTargetwithBlend (Game|GetPlayerController 0) (Variables|Default|GetPlayer) (Variables|Default|GetSmoothProssessDuration) "VTBlend_Linear" 0.0 false)
  (Utilities|FlowControl|Delay (Variables|Default|GetSmoothProssessDuration))
  (Pawn|Possess (Game|GetPlayerController 0) (Variables|Default|GetPlayer))
  (Input|AddMappingContext (PlayerController|LocalPlayerSubsystems|GetEnhancedInputLocalPlayerSubsystem (Game|GetPlayerController 0)) (Variables|Default|GetCharakterMappingContext) 0 "(bIgnoreAllPressedKeysUntilRelease=True,bForceImmediately=False,bNotifyUserSettings=False)"))

(event Custom|Next%20text%20trigger_Event)

(event Input|EnhancedActionEvents|EnhancedInputActionIA_PuzzleEscape
  (params (ActionValue :type Boolean) (ElapsedSeconds :type Float%20%28double-precision%29) (TriggeredSeconds :type Float%20%28double-precision%29) (InputAction :type Input%20Action%20Object%20Reference :default "/Game/Imputs/RätzelInputs/IA_PuzzleEscape.IA_PuzzleEscape"))
  (CallFunction|ReturntoCharacter))

(event EventInteract
  (params (Player :type BP%20Player%20Object%20Reference))
  (bind _output_get (Variables|Default|SetPlayer Player))
  (CallFunction|EventGetPossessed)
  (EventDispatchers|AssignNextTextTrigger (Variables|/Game/BP´s/Player/BP_Player.BP_Player_C|GetMainUI _output_get) (delegate Custom|Next%20text%20trigger_Event)))

(fn ConstructionScript)

(fn PositionPlayerCharacter
  (bind _output_get (LocalVariables|SetCam (Actor|GetComponentbyClass "/Script/Engine.CameraComponent")))
  (Development|PrintString (Utilities|GetDisplayName _output_get))
  (Utilities|IsValid _output_get
    (:Is%20Valid
      (Transformation|SetActorLocation (Variables|Default|GetPlayer) (Math|Vector|MakeVector 0.0 0.0 (.z (Transformation|GetWorldLocation (LocalVariables|GetCam)))) false false)
      (Transformation|SetActorRotation (Variables|Default|GetPlayer) (Math|Rotator|MakeRotator 0.0 0.0 (.yaw (Transformation|GetWorldRotation (LocalVariables|GetCam)))))
      (bind (_outhit _returnvalue) (Collision|LineTraceForObjects (Transformation|GetWorldLocation (LocalVariables|GetCam)) (- (Transformation|GetWorldLocation (LocalVariables|GetCam)) "0.000000,0.000000,600.000000") (Utilities|Array|MakeArray "ObjectTypeQuery1" "ObjectTypeQuery2") false 0 "ForDuration" true "(R=1.000000,G=0.000000,B=0.000000,A=1.000000)" "(R=0.000000,G=1.000000,B=0.000000,A=1.000000)" 1e+01))
      (if _returnvalue
        (Transformation|SetActorLocation (Variables|Default|GetPlayer) (+ (.Location (Collision|BreakHitResult _outhit)) (Math|Vector|MakeVector 0.0 0.0 (+ (Variables|/Script/Engine.CapsuleComponent|GetCapsuleHalfHeight (Variables|/Script/Engine.Character|GetCapsuleComponent (Variables|Default|GetPlayer))) 1.0))) false false)))
    (:Is%20Not%20Valid
      (Development|PrintString "Cam Fehlt" true true "(R=1.000000,G=0.000331,B=0.000000,A=1.000000)" 1e+01))))