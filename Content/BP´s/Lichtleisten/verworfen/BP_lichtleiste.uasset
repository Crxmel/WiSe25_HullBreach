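; Light strip (Lichtleiste) actor, filed under "verworfen" (discarded), that fades five point lights on and off in sequence.
; A delayed Tick calls Lichttrigger, where LightAnimation steps each intensity based on the previous light crossing a percentage threshold, with reversible order.
; Once the last light first steps, later triggers also drive SetNextLight, chaining strips; reaching either limit flips the fade after a delay.
; The sphere-trace neighbour search is unused.
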(event Custom|Lichttrigger
  (bind _pointlight2 (Variables|Default|GetPointLight2))
  (bind _setnextlight (Variables|Default|GetSetNextLight))
  (if (CallFunction|TimeHasPassedSinceLastHits)
    (Variables|Default|SetLastHitTime (Utilities|Time|GetGameTimeinSeconds))
    (Utilities|FlowControl|Sequence
      (:then_0
        (if (Variables|Default|GetSyncroBool)
          (Utilities|IsValid _setnextlight
            (:Is%20Valid
              (CallFunction|Lichttrigger _setnextlight)))))
      (:then_1)
      (:then_2
        (bind (_redy _variablenupdate) (CallFunction|LightAnimation (Variables|einzelneLichtspeicher|GetLight_1) 0.0 5 true))
        (if _redy
          (bind _output_get (Variables|einzelneLichtspeicher|SetLight_1 _variablenupdate))
          (Rendering|Components|Light|SetIntensity (select (Variables|Default|GetLichtLeisteAnRSeite) (Variables|Default|GetPointLight4) (Variables|Default|GetPointLight)) _output_get)))
      (:then_3
        (bind (_redy_2 _variablenupdate_2) (CallFunction|LightAnimation (Variables|einzelneLichtspeicher|GetLight_2) (Variables|einzelneLichtspeicher|GetLight_1) 4 false))
        (if _redy_2
          (bind _output_get_2 (Variables|einzelneLichtspeicher|SetLight_2 _variablenupdate_2))
          (Rendering|Components|Light|SetIntensity (select (Variables|Default|GetLichtLeisteAnRSeite) (Variables|Default|GetPointLight3) (Variables|Default|GetPointLight1)) _output_get_2)))
      (:then_4
        (bind (_redy_3 _variablenupdate_3) (CallFunction|LightAnimation (Variables|einzelneLichtspeicher|GetLight_3) (Variables|einzelneLichtspeicher|GetLight_2) 3 false))
        (if _redy_3
          (bind _output_get_3 (Variables|einzelneLichtspeicher|SetLight_3 _variablenupdate_3))
          (Rendering|Components|Light|SetIntensity (select (Variables|Default|GetLichtLeisteAnRSeite) _pointlight2 _pointlight2) _output_get_3)))
      (:then_5
        (bind (_redy_4 _variablenupdate_4) (CallFunction|LightAnimation (Variables|einzelneLichtspeicher|GetLight_4) (Variables|einzelneLichtspeicher|GetLight_3) 2 false))
        (if _redy_4
          (bind _output_get_4 (Variables|einzelneLichtspeicher|SetLight_4 _variablenupdate_4))
          (Rendering|Components|Light|SetIntensity (select (Variables|Default|GetLichtLeisteAnRSeite) (Variables|Default|GetPointLight1) (Variables|Default|GetPointLight3)) _output_get_4)))
      (:then_6
        (bind (_redy_5 _variablenupdate_5) (CallFunction|LightAnimation (Variables|einzelneLichtspeicher|GetLight_5) (Variables|einzelneLichtspeicher|GetLight_4) 1 false))
        (if _redy_5
          (bind _output_get_5 (Variables|einzelneLichtspeicher|SetLight_5 _variablenupdate_5))
          (Rendering|Components|Light|SetIntensity (select (Variables|Default|GetLichtLeisteAnRSeite) (Variables|Default|GetPointLight) (Variables|Default|GetPointLight4)) _output_get_5)
          (Utilities|FlowControl|Sequence
            (:then_0
              (Variables|Default|SetSyncroBool true))
            (:then_1
              (if (or (<= _output_get_5 0.0) (>= _output_get_5 (Variables|einzelneLichtspeicher|Getlightsave)))
                (if (Variables|Default|Getlightflip)
                  (Utilities|FlowControl|Delay (Variables|Animationgeschwindickkeit|GetLicht%20an%20delay))
                  (else
                    (Utilities|FlowControl|Delay (Variables|Animationgeschwindickkeit|GetLicht%20aus%20delay))))
                (Variables|Default|Setlightflip (not (Variables|Default|Getlightflip)))
                (CallFunction|Reset)))))))))

(event Custom|Reset
  (Utilities|FlowControl|DoOnce false ; enters at Reset
    (:Completed
      (Variables|einzelneLichtspeicher|SetLight_1 (- (Variables|einzelneLichtspeicher|Getlightsave) (* (Variables|Animationgeschwindickkeit|GetÜbergangs%20Steps) 15.0))))))

(event EventBeginPlay
  (Variables|einzelneLichtspeicher|Setlightsave (Variables|/Script/Engine.LightComponentBase|GetIntensity (Variables|Default|GetPointLight)))
  (Variables|Default|SetStart true)
  (bind _output_get (Variables|einzelneLichtspeicher|SetLight_1 (Variables|einzelneLichtspeicher|Getlightsave)))
  (bind _output_get_2 (Variables|einzelneLichtspeicher|SetLight_2 _output_get))
  (bind _output_get_3 (Variables|einzelneLichtspeicher|SetLight_3 _output_get_2))
  (bind _output_get_4 (Variables|einzelneLichtspeicher|SetLight_4 _output_get_3))
  (Variables|einzelneLichtspeicher|SetLight_5 _output_get_4))

(event EventTick
  (params (DeltaSeconds :type Float%20%28single-precision%29))
  (if (Variables|Default|GetligthStart)
    (Utilities|FlowControl|Delay (Variables|Animationgeschwindickkeit|GetAnimationDuration))
    (if (Variables|Default|GetStart)
      (CallFunction|Lichttrigger))))

(fn ConstructionScript)

(fn TimeHasPassedSinceLastHits
  (return (> (Utilities|Time|GetGameTimeinSeconds) (Variables|Default|GetLastHitTime))))

(fn SphereOverlapandSaveActors
  (bind _returnvalue (- 1e+02 0.1))
  (bind _self self)
  (bind _setnextlight (Variables|Default|GetSetNextLight))
  (bind _r_sphere (Variables|Default|GetR_Sphere))
  (bind _returnvalue_2 (Utilities|GetObjectName _self))
  (bind _returnvalue_3 (Transformation|GetWorldLocation _r_sphere))
  (bind (_outhit _returnvalue_4) (Collision|SphereTraceForObjects _returnvalue_3 _returnvalue_3 (Components|Sphere|GetScaledSphereRadius _r_sphere) (Utilities|Array|MakeArray "ObjectTypeQuery1") false 0 "Persistent" false))
  (if _returnvalue_4
    (Development|PrintString (Utilities|GetDisplayName (.HitActor (Collision|BreakHitResult _outhit))))
    (bind _asbp_lichtleiste (Utilities|Casting|CastToBP_lichtleiste (.HitActor (Collision|BreakHitResult _outhit)))
      (:then
        (bind _output_get (Variables|Egalwennfunctionnichttutzt|SetNextLight _asbp_lichtleiste))
        (Development|PrintString (Utilities|String|Append _returnvalue_2 ": cast -->" (Utilities|GetDisplayName _output_get)) true true "(R=0.000000,G=0.660000,B=1.000000,A=1.000000)" _returnvalue)
        (Variables|Default|SetStart true :!label _label))
      (:CastFailed
        (Utilities|IsValid _setnextlight
          (:Is%20Valid
            (bind _output_get_2 (Variables|Egalwennfunctionnichttutzt|SetNextLight _setnextlight))
            (Development|PrintString (Utilities|String|Append _returnvalue_2 ": cast falled -->" (Utilities|GetDisplayName _output_get_2)) true true "(R=0.000000,G=0.660000,B=1.000000,A=1.000000)" _returnvalue)
            (goto _label))
          (:Is%20Not%20Valid
            (Development|PrintString (Utilities|String|Append _returnvalue_2 " : dont set Next Light or Start Light") true true "(R=1.000000,G=0.000000,B=0.025861,A=1.000000)" 1e+02)))))))

(fn LightAnimation
  (params (Change_PointLight_Float :type Float%20%28double-precision%29) (Before_PointLight_float :type Float%20%28double-precision%29) (PointLightNumber_Absteigent :type Integer) (IsTheFirstOne :type Boolean))
  (if (Variables|Default|Getlightflip)
    (if (or (>= Before_PointLight_float (* (Variables|einzelneLichtspeicher|Getlightsave) (/ (Variables|Animationgeschwindickkeit|GetÜbergangsHärte%20in%20%25) 1e+02))) IsTheFirstOne)
      (if (>= Change_PointLight_Float (Variables|einzelneLichtspeicher|Getlightsave))
        (return false 0.0)
        (else
          _))
      (else
        (return false 0.0)))
    (elif (and (<= Before_PointLight_float (* (Variables|einzelneLichtspeicher|Getlightsave) (/ (Variables|Animationgeschwindickkeit|GetÜbergangsHärte%20in%20%25) 1e+02))) (not (<= Change_PointLight_Float 0.0)))
      _
      (else
        (return false 0.0))))
  (return true (Math|Float|SelectFloat (+ Change_PointLight_Float (Variables|Animationgeschwindickkeit|GetÜbergangs%20Steps)) (- Change_PointLight_Float (Variables|Animationgeschwindickkeit|GetÜbergangs%20Steps)) (Variables|Default|Getlightflip))))

(fn LightAnimation0
  (params (Change_PointLight_Float :type Float%20%28double-precision%29) (Before_PointLight_float :type Float%20%28double-precision%29) (PointLightNumber_Absteigent :type Integer) (IsTheFirstOne :type Boolean))
  (if (Variables|Default|Getlightflip)
    (if (or (>= Before_PointLight_float (* (Variables|einzelneLichtspeicher|Getlightsave) (/ (Variables|Animationgeschwindickkeit|GetÜbergangsHärte%20in%20%25) 1e+02))) IsTheFirstOne)
      (if (not (>= Change_PointLight_Float (Variables|einzelneLichtspeicher|Getlightsave)))
        (return true (Math|Float|SelectFloat (+ Change_PointLight_Float (Variables|Animationgeschwindickkeit|GetÜbergangs%20Steps)) (- Change_PointLight_Float (Variables|Animationgeschwindickkeit|GetÜbergangs%20Steps)) (Variables|Default|Getlightflip)))))
    (elif (and (<= Before_PointLight_float (* (Variables|einzelneLichtspeicher|Getlightsave) (/ (Variables|Animationgeschwindickkeit|GetÜbergangsHärte%20in%20%25) 1e+02))) (not (<= Change_PointLight_Float 0.0)))
      (return true (Math|Float|SelectFloat (+ Change_PointLight_Float (Variables|Animationgeschwindickkeit|GetÜbergangs%20Steps)) (- Change_PointLight_Float (Variables|Animationgeschwindickkeit|GetÜbergangs%20Steps)) (Variables|Default|Getlightflip))))))