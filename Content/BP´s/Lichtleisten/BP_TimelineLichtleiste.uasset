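; Light strip of five point lights that plays a running fade and signals an alarm in red.
; Staggered timelines fade the lights out and back in, with OnR reversing the order, switching color to red while faded out or white once the alarm ends.
; The First strip loops while AlarmOn, and each strip passes the state to up to three Next strips.
; Alarm_aus resets a DoOnce so the next cycle clears the alarm.
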(event Custom|Aus%20/%20Trigger%20First
  (bind _next_2 (Variables|Default|Getnext_2))
  (bind _next_3 (Variables|Default|Getnext_3))
  (if (Variables|Default|Getfirst)
    (if (Variables|Default|GetAlarm%20on)
      (Utilities|FlowControl|Sequence
        (:then_0
          (Utilities|FlowControl|Sequence
            (:then_0
              (Utilities|FlowControl|Delay (* (Variables|Mussidentischsein|GetDelay_0,2) 0.0))
              (bind _off (Timeline|Timeline PlayFromStart)
                (:Update
                  (Rendering|Components|Light|SetIntensity (select (Variables|Default|GetonR) (Variables|Default|GetPointLight4) (Variables|Default|GetPointLight)) (* _off (Variables|Mussidentischsein|GetLightIntensety))))
                (:Finished
                  (Utilities|FlowControl|Delay (Variables|Mussidentischsein|GetDuration_an_1,0))
                  (CallFunction|An)
                  (if (Variables|Default|GetAlarm%20on)
                    (Rendering|Components|Light|SetLightColor (Variables|Default|GetPointLight) "(R=1.000000,G=0.000000,B=0.000000,A=1.000000)" true)))))
            (:then_1
              (Utilities|FlowControl|Delay (* (Variables|Mussidentischsein|GetDelay_0,2) 1.0))
              (bind _off_2 (Timeline|Timeline_5 PlayFromStart)
                (:Update
                  (Rendering|Components|Light|SetIntensity (select (Variables|Default|GetonR) (Variables|Default|GetPointLight3) (Variables|Default|GetPointLight1)) (* _off_2 (Variables|Mussidentischsein|GetLightIntensety))))
                (:Finished
                  (if (Variables|Default|GetAlarm%20on)
                    (Rendering|Components|Light|SetLightColor (Variables|Default|GetPointLight1) "(R=1.000000,G=0.000000,B=0.000000,A=1.000000)" true)))))
            (:then_2
              (Utilities|FlowControl|Delay (* (Variables|Mussidentischsein|GetDelay_0,2) 2.0))
              (bind _off_3 (Timeline|Timeline_6 PlayFromStart)
                (:Update
                  (Rendering|Components|Light|SetIntensity (Variables|Default|GetPointLight2) (* _off_3 (Variables|Mussidentischsein|GetLightIntensety))))
                (:Finished
                  (if (Variables|Default|GetAlarm%20on)
                    (Rendering|Components|Light|SetLightColor (Variables|Default|GetPointLight2) "(R=1.000000,G=0.000000,B=0.000000,A=1.000000)" true)))))
            (:then_3
              (Utilities|FlowControl|Delay (* (Variables|Mussidentischsein|GetDelay_0,2) 3.0))
              (bind _off_4 (Timeline|Timeline_7 PlayFromStart)
                (:Update
                  (Rendering|Components|Light|SetIntensity (select (Variables|Default|GetonR) (Variables|Default|GetPointLight1) (Variables|Default|GetPointLight3)) (* _off_4 (Variables|Mussidentischsein|GetLightIntensety))))
                (:Finished
                  (if (Variables|Default|GetAlarm%20on)
                    (Rendering|Components|Light|SetLightColor (Variables|Default|GetPointLight3) "(R=1.000000,G=0.000000,B=0.000000,A=1.000000)" true)))))
            (:then_4
              (Utilities|FlowControl|Delay (* (Variables|Mussidentischsein|GetDelay_0,2) 4.0))
              (Utilities|FlowControl|Sequence
                (:then_0
                  (bind _off_5 (Timeline|Timeline_8 PlayFromStart)
                    (:Update
                      (Rendering|Components|Light|SetIntensity (select (Variables|Default|GetonR) (Variables|Default|GetPointLight) (Variables|Default|GetPointLight4)) (* _off_5 (Variables|Mussidentischsein|GetLightIntensety))))
                    (:Finished
                      (if (Variables|Default|GetAlarm%20on)
                        (Rendering|Components|Light|SetLightColor (Variables|Default|GetPointLight4) "(R=1.000000,G=0.000000,B=0.000000,A=1.000000)" true)))))
                (:then_1
                  (Utilities|IsValid (Variables|Default|Getnext)
                    (:Is%20Valid
                      (Utilities|FlowControl|Delay 0.2)
                      (CallFunction|NextTrigger (Variables|Default|Getnext) (Variables|Default|GetAlarm%20on))
                      (Utilities|IsValid _next_2
                        (:Is%20Valid
                          (CallFunction|NextTrigger _next_2 (Variables|Default|GetAlarm%20on))
                          (Utilities|IsValid _next_3
                            (:Is%20Valid
                              (CallFunction|NextTrigger _next_3 (Variables|Default|GetAlarm%20on)))))))))))))
        (:then_1
          (Utilities|FlowControl|DoOnce true
            (:Completed
              (Variables|Default|SetAlarm%20on false))))))))

(event Custom|Next%20trigger
  (params (NewParam :type Boolean))
  (bind _next_2 (Variables|Default|Getnext_2))
  (bind _next_3 (Variables|Default|Getnext_3))
  (Variables|Default|SetAlarm%20on NewParam)
  (Utilities|FlowControl|Sequence
    (:then_0
      (Utilities|FlowControl|Delay (* (Variables|Mussidentischsein|GetDelay_0,2) 0.0))
      (bind _off (Timeline|Timeline PlayFromStart)
        (:Update
          (Rendering|Components|Light|SetIntensity (select (Variables|Default|GetonR) (Variables|Default|GetPointLight4) (Variables|Default|GetPointLight)) (* _off (Variables|Mussidentischsein|GetLightIntensety))))
        (:Finished
          (Utilities|FlowControl|Delay (Variables|Mussidentischsein|GetDuration_an_1,0))
          (CallFunction|An)
          (if (Variables|Default|GetAlarm%20on)
            (Rendering|Components|Light|SetLightColor (Variables|Default|GetPointLight) "(R=1.000000,G=0.000000,B=0.000000,A=1.000000)" true)))))
    (:then_1
      (Utilities|FlowControl|Delay (* (Variables|Mussidentischsein|GetDelay_0,2) 1.0))
      (bind _off_2 (Timeline|Timeline_5 PlayFromStart)
        (:Update
          (Rendering|Components|Light|SetIntensity (select (Variables|Default|GetonR) (Variables|Default|GetPointLight3) (Variables|Default|GetPointLight1)) (* _off_2 (Variables|Mussidentischsein|GetLightIntensety))))
        (:Finished
          (if (Variables|Default|GetAlarm%20on)
            (Rendering|Components|Light|SetLightColor (Variables|Default|GetPointLight1) "(R=1.000000,G=0.000000,B=0.000000,A=1.000000)" true)))))
    (:then_2
      (Utilities|FlowControl|Delay (* (Variables|Mussidentischsein|GetDelay_0,2) 2.0))
      (bind _off_3 (Timeline|Timeline_6 PlayFromStart)
        (:Update
          (Rendering|Components|Light|SetIntensity (Variables|Default|GetPointLight2) (* _off_3 (Variables|Mussidentischsein|GetLightIntensety))))
        (:Finished
          (if (Variables|Default|GetAlarm%20on)
            (Rendering|Components|Light|SetLightColor (Variables|Default|GetPointLight2) "(R=1.000000,G=0.000000,B=0.000000,A=1.000000)" true)))))
    (:then_3
      (Utilities|FlowControl|Delay (* (Variables|Mussidentischsein|GetDelay_0,2) 3.0))
      (bind _off_4 (Timeline|Timeline_7 PlayFromStart)
        (:Update
          (Rendering|Components|Light|SetIntensity (select (Variables|Default|GetonR) (Variables|Default|GetPointLight1) (Variables|Default|GetPointLight3)) (* _off_4 (Variables|Mussidentischsein|GetLightIntensety))))
        (:Finished
          (if (Variables|Default|GetAlarm%20on)
            (Rendering|Components|Light|SetLightColor (Variables|Default|GetPointLight3) "(R=1.000000,G=0.000000,B=0.000000,A=1.000000)" true)))))
    (:then_4
      (Utilities|FlowControl|Delay (* (Variables|Mussidentischsein|GetDelay_0,2) 4.0))
      (Utilities|FlowControl|Sequence
        (:then_0
          (bind _off_5 (Timeline|Timeline_8 PlayFromStart)
            (:Update
              (Rendering|Components|Light|SetIntensity (select (Variables|Default|GetonR) (Variables|Default|GetPointLight) (Variables|Default|GetPointLight4)) (* _off_5 (Variables|Mussidentischsein|GetLightIntensety))))
            (:Finished
              (if (Variables|Default|GetAlarm%20on)
                (Rendering|Components|Light|SetLightColor (Variables|Default|GetPointLight4) "(R=1.000000,G=0.000000,B=0.000000,A=1.000000)" true)))))
        (:then_1
          (Utilities|IsValid (Variables|Default|Getnext)
            (:Is%20Valid
              (Utilities|FlowControl|Delay 0.2)
              (CallFunction|NextTrigger (Variables|Default|Getnext) (Variables|Default|GetAlarm%20on))
              (Utilities|IsValid _next_2
                (:Is%20Valid
                  (CallFunction|NextTrigger _next_2 (Variables|Default|GetAlarm%20on))
                  (Utilities|IsValid _next_3
                    (:Is%20Valid
                      (CallFunction|NextTrigger _next_3 (Variables|Default|GetAlarm%20on)))))))))))))

(event Custom|An
  (Utilities|FlowControl|Sequence
    (:then_0
      (Utilities|FlowControl|Delay (* (Variables|Mussidentischsein|GetDelay_0,2) 0.0))
      (if (Variables|Default|GetAlarm%20on)
        (bind _on (Timeline|Timeline_0 PlayFromStart)
          (:Update
            (Rendering|Components|Light|SetIntensity (select (Variables|Default|GetonR) (Variables|Default|GetPointLight4) (Variables|Default|GetPointLight)) (* _on (Variables|Mussidentischsein|GetLightIntensety))))
          (:Finished
            (Utilities|FlowControl|Delay (Variables|Mussidentischsein|GetDuration_aus_0,0))
            (if (Variables|Default|GetAlarm%20on)
              (CallFunction|Aus/TriggerFirst))))
        (else
          (Rendering|Components|Light|SetLightColor (Variables|Default|GetPointLight) "(R=1.000000,G=1.000000,B=1.000000,A=1.000000)" true)
          (Timeline|Timeline_0 PlayFromStart))))
    (:then_1
      (Utilities|FlowControl|Delay (* (Variables|Mussidentischsein|GetDelay_0,2) 1.0))
      (if (Variables|Default|GetAlarm%20on)
        (bind _on_2 (Timeline|Timeline_1 PlayFromStart)
          (:Update
            (Rendering|Components|Light|SetIntensity (select (Variables|Default|GetonR) (Variables|Default|GetPointLight3) (Variables|Default|GetPointLight1)) (* _on_2 (Variables|Mussidentischsein|GetLightIntensety)))))
        (else
          (Rendering|Components|Light|SetLightColor (Variables|Default|GetPointLight1) "(R=1.000000,G=1.000000,B=1.000000,A=1.000000)" true)
          (Timeline|Timeline_1 PlayFromStart))))
    (:then_2
      (Utilities|FlowControl|Delay (* (Variables|Mussidentischsein|GetDelay_0,2) 2.0))
      (if (Variables|Default|GetAlarm%20on)
        (bind _on_3 (Timeline|Timeline_2 PlayFromStart)
          (:Update
            (Rendering|Components|Light|SetIntensity (Variables|Default|GetPointLight2) (* _on_3 (Variables|Mussidentischsein|GetLightIntensety)))))
        (else
          (Rendering|Components|Light|SetLightColor (Variables|Default|GetPointLight2) "(R=1.000000,G=1.000000,B=1.000000,A=1.000000)" true)
          (Timeline|Timeline_2 PlayFromStart))))
    (:then_3
      (Utilities|FlowControl|Delay (* (Variables|Mussidentischsein|GetDelay_0,2) 3.0))
      (if (Variables|Default|GetAlarm%20on)
        (bind _on_4 (Timeline|Timeline_3 PlayFromStart)
          (:Update
            (Rendering|Components|Light|SetIntensity (select (Variables|Default|GetonR) (Variables|Default|GetPointLight1) (Variables|Default|GetPointLight3)) (* _on_4 (Variables|Mussidentischsein|GetLightIntensety)))))
        (else
          (Rendering|Components|Light|SetLightColor (Variables|Default|GetPointLight3) "(R=1.000000,G=1.000000,B=1.000000,A=1.000000)" true)
          (Timeline|Timeline_3 PlayFromStart))))
    (:then_4
      (Utilities|FlowControl|Delay (* (Variables|Mussidentischsein|GetDelay_0,2) 4.0))
      (if (Variables|Default|GetAlarm%20on)
        (bind _on_5 (Timeline|Timeline_4 PlayFromStart)
          (:Update
            (Rendering|Components|Light|SetIntensity (select (Variables|Default|GetonR) (Variables|Default|GetPointLight) (Variables|Default|GetPointLight4)) (* _on_5 (Variables|Mussidentischsein|GetLightIntensety)))))
        (else
          (Rendering|Components|Light|SetLightColor (Variables|Default|GetPointLight4) "(R=1.000000,G=1.000000,B=1.000000,A=1.000000)" true)
          (Timeline|Timeline_4 PlayFromStart))))))

(event Custom|Alarm_an
  (Variables|Default|SetAlarm%20on true)
  (CallFunction|Aus/TriggerFirst))

(event Custom|Alarm_aus
  (Utilities|FlowControl|DoOnce true) ; enters at Reset
)

(event EventBeginPlay
  (Variables|Mussidentischsein|SetLightIntensety (Variables|/Script/Engine.LightComponentBase|GetIntensity (Variables|Default|GetPointLight)))
  (CallFunction|Aus/TriggerFirst))

(fn ConstructionScript
  (Rendering|Components|Light|SetIntensity (Variables|Default|GetPointLight1) (select (Variables|customizeinBP|Getcostomize%20light) (Variables|customizeinBP|GetLight%20Intensety) 0.0)))